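; Game mode for the first arena, gating progression to Arena002 on clearing the enemies and then hitting the statue.
; Every tick it counts BP_Charger actors; when none remain, it flags BP_Statue as vulnerable and swaps its material.
; The same tick polls the statue's GotHit flag and opens Arena002 once it is set.
; State is found by per-frame actor lookups, so the vulnerable setup reapplies every frame after the clear.
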(event EventBeginPlay)

(event EventTick
  (params (DeltaSeconds :type Float%20%28single-precision%29))
  (Utilities|FlowControl|Sequence
    (:then_0
      (bind _allenemiesdead (CallFunction|CheckEnemyCount))
      (if _allenemiesdead
        (CallFunction|SetStatueVulnerable)))
    (:then_1
      (bind _returnvalue (Actor|GetActorOfClass "/Game/EdgeOfSorrow/Blueprints/Items/BP_Statue.BP_Statue_C"))
      (Utilities|IsValid _returnvalue
        (:Is%20Valid
          (if (Variables|/Game/EdgeOfSorrow/Blueprints/Items/BP_Statue.BP_Statue_C|GetGotHit _returnvalue)
            (Game|OpenLevel(byObjectReference) "/Game/EdgeOfSorrow/Maps/Arena002.Arena002")))))))

(fn ConstructionScript)

(fn CheckEnemyCount
  (bind _outactors (Actor|GetAllActorsOfClass "/Game/EdgeOfSorrow/Blueprints/Enemies/BP_Charger.BP_Charger_C"))
  (return (<= (Utilities|Array|Length _outactors) 0)))

(fn SetStatueVulnerable
  (bind _returnvalue (Actor|GetActorOfClass "/Game/EdgeOfSorrow/Blueprints/Items/BP_Statue.BP_Statue_C"))
  (Utilities|IsValid _returnvalue
    (:Is%20Valid
      (Rendering|Material|SetMaterial (Variables|/Game/EdgeOfSorrow/Blueprints/Items/BP_Statue.BP_Statue_C|GetSM_Statue03 _returnvalue) 0 "/Game/EdgeOfSorrow/Materials/Colors/M_CelColor7.M_CelColor7")
      (Variables|/Game/EdgeOfSorrow/Blueprints/Items/BP_Statue.BP_Statue_C|SetIsVunerable _returnvalue true))))