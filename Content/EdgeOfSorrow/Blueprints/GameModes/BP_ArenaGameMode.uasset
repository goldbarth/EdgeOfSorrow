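; Arena game mode that runs numbered enemy waves through doll head spawners and opens an exit portal when the round ends.
; Each wave builds an enemy pool from a data table row, or random counts if none exists, then queues a capped batch at random spawners.
; Defeats refill spawners from the pool until a timer starts the next wave.
; RoundEnd line-traces ahead of the player to place a portal facing them.
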(event Custom|RoundEnd
  ;[0 0 0] On Round End
  (Utilities|FlowControl|Delay 3.0)
  (CallFunction|SpawnExit "/Game/EdgeOfSorrow/Blueprints/Environment/ExitPortal/BP_SpawnableExitPortal.BP_SpawnableExitPortal_C"))

(event EventBeginPlay
  (Utilities|FlowControl|Sequence
    (:then_0
      (CallFunction|SetWaveController))
    (:then_1
      (CallFunction|SetFirstPersonCharacter))
    (:then_2
      ;[0 0 0] Source: Wave Mode Tutorial @ Ryan Laley (YT)
      (Utilities|FlowControl|Delay 2.0)
      (CallFunction|GetSpawners)
      (CallFunction|NewWave))))

(fn ConstructionScript)

(fn GetSpawners
  (bind _outactors (Actor|GetAllActorsOfClass "/Game/EdgeOfSorrow/Blueprints/Enemies/BP_DollHeadSpawner.BP_DollHeadSpawner_C"))
  (Variables|Default|SetSpawners _outactors))

(fn StartWave
  (bind _spawners (Variables|Default|GetSpawners))
  (bind _outitem (Utilities|Array|Random _spawners))
  (CallFunction|BuildEnemyPool)
  (for _index (range 0 (- (Math|Integer|Min(Integer) (CallFunction|GetPoolsize) (Variables|Default|GetEnemyMaxCount)) 1))
    (bind _enemyclass (CallFunction|GetEnemyfromPool))
    (Utilities|IsValid _outitem
      (:Is%20Valid
        (Default|AddEnemytoQueue _outitem _enemyclass)))))

(fn EndWave)

(fn EnterTransition
  (params (TransitionPeriod :type Float%20%28single-precision%29))
  (bind _returnvalue (Utilities|Time|SetTimerbyFunctionName 0 "NewWave" TransitionPeriod))
  (Variables|Default|SetTransitionTimer _returnvalue))

(fn BuildEnemyPool
  (bind _returnvalue (Utilities|GetDataTableRow "/Game/EdgeOfSorrow/Blueprints/Enemies/DT_WavePoolData.DT_WavePoolData" (Utilities|String|StringToName (Utilities|String|ToString(Integer) (Variables|Default|GetWaveNumber))))
    (:then
      (bind _output_get (Variables|Default|SetEnemyPool (Utilities|Struct|BreakF_WaveStruct _returnvalue)))
      (Development|PrintString (Utilities|String|ToString(Integer) (Utilities|Map|Length _output_get)) true true "(R=0.000000,G=0.660000,B=1.000000,A=1.000000)" 1e+01))
    (:RowNotFound
      (Utilities|Map|Add (Variables|Default|GetEnemyPool) "/Game/EdgeOfSorrow/Blueprints/Enemies/BP_DollHead.BP_DollHead_C" (Math|Random|RandomIntegerinRange (Variables|Default|GetMinEnemyCount) (* (Variables|Default|GetWaveNumber) 5)))
      (Utilities|Map|Add (Variables|Default|GetEnemyPool) "/Game/EdgeOfSorrow/Blueprints/Enemies/BP_DollHead_Child.BP_DollHead_Child_C" (Math|Random|RandomIntegerinRange (Variables|Default|GetMinEnemyChildCount) (* (Variables|Default|GetWaveNumber) 3)))))
  (Variables|Default|SetEnemyRemaining (CallFunction|GetPoolsize)))

(fn GetPoolsize
  (bind _values (Utilities|Map|Values (Variables|Default|GetEnemyPool)))
  (for _array_element _values
    (bind _output_get (LocalVariables|SetLocalSum (+ (LocalVariables|GetLocalSum) _array_element))))
  (return _output_get))

(fn GetEnemyfromPool
  (bind _keys (Utilities|Map|Keys (Variables|Default|GetEnemyPool)))
  (bind _output_get (LocalVariables|SetClassChoice (.OutItem (Utilities|Array|Random _keys))))
  (if (> (- (.Value (Utilities|Map|Find (Variables|Default|GetEnemyPool) _output_get)) 1) 0)
    (Utilities|Map|Add (Variables|Default|GetEnemyPool) (LocalVariables|GetClassChoice) (- (.Value (Utilities|Map|Find (Variables|Default|GetEnemyPool) _output_get)) 1))
    (else
      (Utilities|Map|Remove (Variables|Default|GetEnemyPool) (LocalVariables|GetClassChoice))))
  (return (LocalVariables|GetClassChoice)))

(fn NewWave
  (Math|Integer|IncrementInt (Variables|Default|GetWaveNumber)
    (:%20%20
      (CallFunction|StartWave))))

(fn OnEnemyDefeated
  (bind _spawners (Variables|Default|GetSpawners))
  (bind _outitem (Utilities|Array|Random _spawners))
  (bind _result (Math|Integer|DecrementInt (Variables|Default|GetEnemyRemaining))
    (:%20%20
      (if (< _result (Variables|Default|GetEnemyMaxCount))
        (if (<= (Variables|Default|GetEnemyRemaining) 0)
          (CallFunction|EnterTransition (Variables|Default|GetTransitionWavePeriod)))
        (else
          (bind _enemyclass (CallFunction|GetEnemyfromPool))
          (Utilities|IsValid _outitem
            (:Is%20Valid
              (Default|AddEnemytoQueue _outitem _enemyclass))))))))

(fn SetFirstPersonCharacter
  (bind _returnvalue (Game|GetPlayerCharacter 0))
  (bind _asbp_first_person_character (Utilities|Casting|CastToBP_FirstPersonCharacter _returnvalue))
  (Utilities|IsValid _asbp_first_person_character
    (:Is%20Valid
      (Variables|Default|SetFirstPersonCharacter _asbp_first_person_character))))

(fn SpawnExit
  (params (ExitActor :type Actor%20Class%20Reference))
  (bind _distancetocircleexit (Variables|Default|GetDistanceToCircleExit))
  (bind _firstpersoncharacter (Variables|Default|GetFirstPersonCharacter))
  (bind _returnvalue (Transformation|GetActorForwardVector _firstpersoncharacter))
  (bind _returnvalue_2 (Transformation|GetActorLocation _firstpersoncharacter))
  (bind _returnvalue_3 (* _returnvalue _distancetocircleexit))
  (bind _returnvalue_4 (+ _returnvalue_3 _returnvalue_2))
  (LocalVariables|SetSpawnActor ExitActor)
  (Utilities|IsValid _firstpersoncharacter
    (:Is%20Valid
      ;[0 0 0] Calculate the Distance to the Ground
      (bind _outhit (Collision|LineTraceByChannel _returnvalue_4 (+ _returnvalue_4 (Variables|Default|GetGroundDetectionDistance)) "TraceTypeQuery1" false 0 "ForOneFrame"))
      (bind _returnvalue_5 (Game|SpawnActorfromClass (LocalVariables|GetSpawnActor) (Math|Conversions|ToTransform(Vector) (.ImpactPoint (Collision|BreakHitResult _outhit))) "Undefined" "MultiplyWithRoot" 0 0))
      ;[0 0 0] Face the front always to the Player
      (Transformation|SetActorRotation _returnvalue_5 (Math|Rotator|FindLookatRotation (Transformation|GetActorLocation _returnvalue_5) (Transformation|GetActorLocation (Variables|Default|GetFirstPersonCharacter))))
      (bind _outactors (Actor|GetAllActorsOfClass "/Game/EdgeOfSorrow/Blueprints/PostProcessVolumes/BP_MixedPPV.BP_MixedPPV_C"))
      (if (Utilities|Array|IsEmpty _outactors)
        _
        (else
          (Utilities|IsValid (Utilities|Array|Get(acopy) _outactors)
            (:Is%20Valid
              (Default|SwitchLightPosition (Utilities|Array|Get(acopy) _outactors)))
            (:Is%20Not%20Valid
              _))))
      (Audio|PlaySound2D "/Game/EdgeOfSorrow/Audio/ZapSplat/SW_zapsplat_multimedia_game_sound_win_coins_award_hit_74540_Cue.SW_zapsplat_multimedia_game_sound_win_coins_award_hit_74540_Cue" 1.0 1.0 0.0 0 0))))

(fn SetWaveController
  (bind _returnvalue (Actor|GetActorOfClass "/Game/EdgeOfSorrow/Blueprints/WaveSystem/BP_WaveController.BP_WaveController_C"))
  (Utilities|IsValid _returnvalue
    (:Is%20Valid
      (Variables|Default|SetWaveController _returnvalue))))