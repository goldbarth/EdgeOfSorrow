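; Game mode for Arena002 that runs endless waves of enemies, starting shortly after play begins.
; Each wave totals the EnemyPool counts and queues enemies up to EnemyMaxCount on randomly picked BP_EnemySpawner actors.
; OnEnemyDefeated queues replacements while enough remain, then sets a timer to start the next wave at zero.
; The pool only sets wave size, as every enemy is BP_DollHead; EndWave is empty.
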(event EventBeginPlay
  ;[0 0 0] Source: Wave Mode Tutorial @ Ryan Laley (YT)
  (Utilities|FlowControl|Delay 2.0)
  (CallFunction|GetSpawners)
  (CallFunction|NewWave))

(fn ConstructionScript)

(fn GetSpawners
  (bind _outactors (Actor|GetAllActorsOfClass "/Game/EdgeOfSorrow/Blueprints/Enemies/BP_EnemySpawner.BP_EnemySpawner_C"))
  (Variables|Default|SetSpawners _outactors))

(fn StartWave
  (bind _spawners (Variables|Default|GetSpawners))
  (bind _outitem (Utilities|Array|Random _spawners))
  (CallFunction|BuildEnemyPool)
  (for _index (range 0 (- (Math|Integer|Min(Integer) (CallFunction|GetPoolsize) (Variables|Default|GetEnemyMaxCount)) 1))
    (bind _enemyclass (CallFunction|GetEnemyfromPool))
    (Utilities|IsValid _outitem
      (:Is%20Valid
        (Default|AddEnemytoQueue _outitem _enemyclass))
      (:Is%20Not%20Valid
        (Development|PrintString "Prevent spawning \"DollHeads\" bc no enemy spawner in scene." true true "(R=1.000000,G=0.808392,B=0.000000,A=1.000000)")))))

(fn EndWave)

(fn EnterTransition
  (params (TransitionPeriod :type Float%20%28single-precision%29))
  (bind _returnvalue (Utilities|Time|SetTimerbyFunctionName 0 "NewWave" TransitionPeriod))
  (Variables|Default|SetTransitionTimer _returnvalue))

(fn BuildEnemyPool
  (Variables|Default|SetEnemyRemaining (CallFunction|GetPoolsize)))

(fn GetPoolsize
  (bind _values (Utilities|Map|Values (Variables|Default|GetEnemyPool)))
  (for _array_element _values
    (LocalVariables|SetLocalSum (+ (LocalVariables|GetLocalSum) _array_element)))
  (return (LocalVariables|GetLocalSum)))

(fn GetEnemyfromPool
  (return "/Game/EdgeOfSorrow/Blueprints/Enemies/BP_DollHead.BP_DollHead_C"))

(fn NewWave
  (Math|Integer|IncrementInt (Variables|Default|GetWaveNumber)
    (:%20%20
      (CallFunction|StartWave))))

(fn OnEnemyDefeated
  (bind _result (Math|Integer|DecrementInt (Variables|Default|GetEnemyRemaining))
    (:%20%20
      (if (< _result (Variables|Default|GetEnemyMaxCount))
        (if (<= (Variables|Default|GetEnemyRemaining) 0)
          (CallFunction|EnterTransition (Variables|Default|GetTransitionWavePeriod)))
        (else
          (bind _enemyclass (CallFunction|GetEnemyfromPool))
          (Default|AddEnemytoQueue (.OutItem (Utilities|Array|Random (Variables|Default|GetSpawners))) _enemyclass))))))