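; BP_DollHead is an enemy pawn that chases seen pawns and damages the first-person character on capsule contact.
; Sightings start an AI chase and refresh a short retriggerable delay, which switches to random roaming once sightings lapse.
; Roaming repeats after each successful move but is not started on BeginPlay.
; Any damage kills it instantly, spawning an upgrade orb and calling the enemy-destroyed notification.
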(event OnComponentHit(CapsuleComponent)
  (params (HitComponent :type Primitive%20Component%20Object%20Reference) (OtherActor :type Actor%20Object%20Reference) (OtherComp :type Primitive%20Component%20Object%20Reference) (NormalImpulse :type Vector :default "0, 0, 0") (Hit :type Hit%20Result%20Structure%20%28by%20ref%29))
  ;[0 0 0] Do Damage
  (bind _asbp_first_person_character (Utilities|Casting|CastToBP_FirstPersonCharacter OtherActor))
  (Game|Damage|ApplyDamage _asbp_first_person_character 1.0 0 0))

(event OnSeePawn(PawnSensing)
  (params (Pawn :type Pawn%20Object%20Reference))
  ;[0 0 0] Chase and Roam
  (Utilities|FlowControl|Sequence
    (:then_0
      (AI|AIMoveTo self "0, 0, 0" Pawn 5.0 false))
    (:then_1
      (Utilities|FlowControl|RetriggerableDelay 0.6)
      (CallFunction|Move))))

(event Custom|Move
  ;[0 0 0] AI-Roam Logic
  (AI|AIMoveTo self (.RandomLocation (AI|Navigation|GetRandomReachablePointinRadius (Transformation|GetActorLocation) 5e+03 0 0)) 0 5.0 false
    (:OnSuccess
      (Utilities|FlowControl|Delay 3.0)
      (CallFunction|Move))))

(event EventBeginPlay
  ;[0 0 0] AI-Roam Logic
)

(event Game|Damage|EventAnyDamage
  (params (Damage :type Float%20%28single-precision%29) (DamageType :type Damage%20Type%20Object%20Reference) (InstigatedBy :type Controller%20Object%20Reference) (DamageCauser :type Actor%20Object%20Reference))
  ;[0 0 0] On Take Damage
  (CallFunction|SpawnUpgradeOrb)
  (Actor|DestroyActor)
  (Default|CallOnEnemyDestroyed))

(fn ConstructionScript)

(fn SpawnUpgradeOrb
  (Game|SpawnActorfromClass "/Game/EdgeOfSorrow/Blueprints/BP_UpgradeOrb.BP_UpgradeOrb_C" (Transformation|GetActorTransform) "Undefined" "MultiplyWithRoot" 0 0))