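; Base enemy character that chases the first-person player, damages them, and drops a pickup when it dies.
; On BeginPlay it caches game references and starts an AI MoveTo loop that re-issues shortly after each success or failure.
; Helpers subtract health and apply damage to the player while the enemy is alive.
; Death halts movement, waits out the animation, spawns a coin or upgrade orb based on GameInstance's death count, increments it, then destroys the actor.
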(event Custom|OnDeath
  ;[0 0 0] On Death
  (Variables|Default|SetIsDead true)
  (Components|Movement|StopMovementImmediately (Variables|Character|GetCharacterMovement))
  (Utilities|FlowControl|Delay (Variables|Default|GetDeathAnimationDuration))
  (CallFunction|InitializeDeath))

(event Custom|MoveToTargetImediatly
  ;[0 0 0] Chase
  (AI|AIMoveTo self "0, 0, 0" (Variables|Default|GetFirstPersonCharacter) 5.0 false :!label _label
    (:OnSuccess
      _)
    (:OnFail
      _))
  (Utilities|FlowControl|Delay 0.2)
  (goto _label))

(event EventBeginPlay
  ;[0 0 0] Initialize
  (Utilities|FlowControl|Sequence
    (:then_0
      (CallFunction|SetGameInstance))
    (:then_1
      (CallFunction|SetGameMode))
    (:then_2
      (CallFunction|SetFirstPersonCharacter))
    (:then_3
      (CallFunction|MovetoTargetImediatly))))

(fn ConstructionScript)

(fn SetFirstPersonCharacter
  (bind _returnvalue (Game|GetPlayerCharacter 0))
  (bind _asbp_first_person_character (Utilities|Casting|CastToBP_FirstPersonCharacter _returnvalue))
  (Utilities|IsValid _asbp_first_person_character
    (:Is%20Valid
      (Variables|Default|SetFirstPersonCharacter _asbp_first_person_character))))

(fn SetGameMode
  (bind _returnvalue (Game|GetGameMode))
  (bind _asbp_arena_game_mode (Utilities|Casting|CastToBP_ArenaGameMode _returnvalue))
  (Utilities|IsValid _asbp_arena_game_mode
    (:Is%20Valid
      (Variables|Default|SetArenaGameMode _asbp_arena_game_mode))))

(fn DoDamage
  (params (OtherActor :type Actor%20Object%20Reference))
  (bind _asbp_first_person_character (Utilities|Casting|CastToBP_FirstPersonCharacter OtherActor))
  (if (not (Variables|Default|GetIsDead))
    (Utilities|IsValid _asbp_first_person_character
      (:Is%20Valid
        (Game|Damage|ApplyDamage _asbp_first_person_character (Variables|Default|GetDamage) 0 0)))))

(fn UpdateHealth
  (params (Damage :type Float%20%28double-precision%29))
  (bind _output_get (Variables|Default|SetHealth (- (Variables|Default|GetHealth) Damage)))
  (return _output_get))

(fn InitializeDeath
  (bind _gameinstance (Variables|Default|GetGameInstance))
  (bind _enemydeathcount (Variables|/Game/EdgeOfSorrow/Blueprints/BP_GameInstance.BP_GameInstance_C|GetEnemyDeathCount _gameinstance))
  (Utilities|IsValid _gameinstance
    (:Is%20Valid
      (if (and (!= _enemydeathcount 0) (== (Math|Integer|%(Integer) _enemydeathcount (Variables|Default|GetCoinSpawnDeathNumber)) 0))
        (CallFunction|SpawnCoin)
        (else
          (CallFunction|SpawnUpgradeOrb)))
      (CallFunction|UpdateDeathCount)
      (Actor|DestroyActor))))

(fn SpawnUpgradeOrb
  (Game|SpawnActorfromClass "/Game/EdgeOfSorrow/Blueprints/Collectibles/BP_UpgradeOrb.BP_UpgradeOrb_C" (Transformation|GetActorTransform) "Undefined" "MultiplyWithRoot" 0 0))

(fn SpawnCoin
  (Game|SpawnActorfromClass "/Game/EdgeOfSorrow/Blueprints/Collectibles/BP_Coin.BP_Coin_C" (Transformation|GetActorTransform) "Undefined" "MultiplyWithRoot" 0 0))

(fn UpdateDeathCount
  (bind _gameinstance (Variables|Default|GetGameInstance))
  (Utilities|IsValid _gameinstance
    (:Is%20Valid
      (bind _result (Math|Integer|IncrementInt (Variables|/Game/EdgeOfSorrow/Blueprints/BP_GameInstance.BP_GameInstance_C|GetEnemyDeathCount _gameinstance))
        (:%20%20
          (Variables|/Game/EdgeOfSorrow/Blueprints/BP_GameInstance.BP_GameInstance_C|SetEnemyDeathCount (Variables|Default|GetGameInstance) _result))))))

(fn SetGameInstance
  (bind _returnvalue (Game|GetGameInstance))
  (bind _asbp_game_instance (Utilities|Casting|CastToBP_GameInstance _returnvalue))
  (Utilities|IsValid _asbp_game_instance
    (:Is%20Valid
      (Variables|Default|SetGameInstance _asbp_game_instance))))