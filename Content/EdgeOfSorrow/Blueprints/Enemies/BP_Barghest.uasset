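; BP_Barghest is an enemy Blueprint that deals contact damage and can be killed.
; Each tick it sets IsTargetInRange by comparing its distance to FirstPersonCharacter against AttackDistance.
; Capsule hits pass the other actor to DoDamage, without checking that range flag.
; Incoming damage runs through UpdateHealth and triggers OnDeath at zero or below; these functions are defined outside this file.
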(event OnComponentHit(CapsuleComponent)
  (params (HitComponent :type Primitive%20Component%20Object%20Reference) (OtherActor :type Actor%20Object%20Reference) (OtherComp :type Primitive%20Component%20Object%20Reference) (NormalImpulse :type Vector :default "0, 0, 0") (Hit :type Hit%20Result%20Structure%20%28by%20ref%29))
  ;[0 0 0] Do Damage
  (CallFunction|DoDamage OtherActor))

(event EventTick
  (params (DeltaSeconds :type Float%20%28single-precision%29))
  (CallFunction|CheckTargetRange))

(event Game|Damage|EventAnyDamage
  (params (Damage :type Float%20%28single-precision%29) (DamageType :type Damage%20Type%20Object%20Reference) (InstigatedBy :type Controller%20Object%20Reference) (DamageCauser :type Actor%20Object%20Reference))
  ;[0 0 0] On Take Damage
  (bind _health (CallFunction|UpdateHealth Damage))
  (if (<= _health 0.0)
    (CallFunction|OnDeath)))

(fn ConstructionScript)

(fn CheckTargetRange
  (bind _firstpersoncharacter (Variables|Default|GetFirstPersonCharacter))
  (Utilities|IsValid _firstpersoncharacter
    (:Is%20Valid
      (if (<= (Transformation|GetDistanceTo _firstpersoncharacter self) (Variables|Default|GetAttackDistance))
        (Variables|Default|SetIsTargetInRange true)
        (else
          (Variables|Default|SetIsTargetInRange false))))))