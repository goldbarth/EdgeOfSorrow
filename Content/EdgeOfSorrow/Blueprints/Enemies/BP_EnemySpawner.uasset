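; Destructible enemy spawner that works through a queue of enemy classes and acts as the win objective.
; A looping timer spawns the front entry after a short startup delay, and newly queued enemies trigger an immediate attempt if no BP_DollHead overlaps the capsule.
; Spawned enemies get a destroyed-event binding, and defeats are forwarded to BP_Arena002GameMode.
; Depleting its health destroys it, pauses the game and shows the win screen.
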(event Custom|OnEnemyDefeated
  ;[0 0 0] Update the Enemy Queue
  (bind _asbp_arena_002game_mode (Utilities|Casting|CastToBP_Arena002GameMode (Game|GetGameMode)))
  (Default|OnEnemyDefeated _asbp_arena_002game_mode))

(event Custom|TryToSpawn
  ;[0 0 0] Spawn loop
  (CallFunction|SpawnEnemy))

(event EventBeginPlay
  ;[0 0 0] Spawn loop
  (Utilities|FlowControl|Delay 2.1)
  (Utilities|Time|SetTimerbyEvent (delegate Custom|TryToSpawn) 3.0 true))

(event Game|Damage|EventAnyDamage
  (params (Damage :type Float%20%28single-precision%29) (DamageType :type Damage%20Type%20Object%20Reference) (InstigatedBy :type Controller%20Object%20Reference) (DamageCauser :type Actor%20Object%20Reference))
  ;[0 0 0] Damage logic
  (bind _isdestroyed (CallFunction|TakeDamage Damage))
  (if _isdestroyed
    (Utilities|FlowControl|Sequence
      (:then_0
        (Actor|DestroyActor))
      (:then_1
        (Game|SetGamePaused true)
        (Viewport|RemoveAllWidgets)
        (bind _returnvalue (UserInterface|CreateWidget "/Game/EdgeOfSorrow/UI/Game/WB_WinScreen.WB_WinScreen_C"))
        (UserInterface|Viewport|AddtoViewport _returnvalue 0)))))

(fn ConstructionScript)

(fn SpawnEnemy
  ;[0 0 0] Spawns enemies in the right time
  (if (Utilities|Array|IsValidIndex (Variables|Default|GetEnemyQueue))
    (bind _returnvalue (Game|SpawnActorfromClass (Utilities|Array|Get(acopy) (Variables|Default|GetEnemyQueue)) (Transformation|GetActorTransform) "Undefined" "MultiplyWithRoot" 0 0))
    (Utilities|IsValid _returnvalue
      (:Is%20Valid
        (EventDispatchers|BindEventtoOnEnemyDestroyed _returnvalue (EventDispatchers|CreateEvent :!event Custom|OnEnemyDefeated))
        (Utilities|Array|RemoveIndex (Variables|Default|GetEnemyQueue))
        (return true)))
    (else
      (return false))))

(fn AddEnemytoQueue
  (params (EnemyClass :type BP%20Doll%20Head%20Class%20Reference%20%28by%20ref%29))
  (Utilities|Array|Add (Variables|Default|GetEnemyQueue) EnemyClass)
  (if (not (Utilities|Array|IsValidIndex (Collision|GetOverlappingActors (Variables|Default|GetCapsuleCollision) "/Game/EdgeOfSorrow/Blueprints/Enemies/BP_DollHead.BP_DollHead_C" :!class /Script/Engine.PrimitiveComponent)))
    (CallFunction|SpawnEnemy)))

(fn TakeDamage
  (params (Damage :type Float%20%28double-precision%29))
  (Variables|Default|SetHealth (Math|Float|Truncate (- (Variables|Default|GetHealth) Damage)))
  (return (<= (Variables|Default|GetHealth) 0)))