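; BP_Large is an enemy that chases pawns it sees and dies from any damage.
; PawnSensing drives the AI move, and a retriggerable delay switches it to looping random roaming once sightings stop.
; Capsule hits damage the first-person character, while taking damage briefly delays, spawns an upgrade orb and destroys the enemy.
; Tick sets an in-range flag when the cached player is within attack distance, never clearing it here.
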(event OnComponentHit(CapsuleComponent)
  (params (HitComponent :type Primitive%20Component%20Object%20Reference) (OtherActor :type Actor%20Object%20Reference) (OtherComp :type Primitive%20Component%20Object%20Reference) (NormalImpulse :type Vector :default "0, 0, 0") (Hit :type Hit%20Result%20Structure%20%28by%20ref%29))
  (bind _asbp_first_person_character (Utilities|Casting|CastToBP_FirstPersonCharacter OtherActor))
  ;[0 0 0] Do Damage
  (if (not (Variables|Default|GetIsDead))
    (Utilities|IsValid _asbp_first_person_character
      (:Is%20Valid
        (Game|Damage|ApplyDamage _asbp_first_person_character 1.0 0 0)))))

(event OnSeePawn(PawnSensing)
  (params (Pawn :type Pawn%20Object%20Reference))
  ;[0 0 0] Chase and Roam
  (if (not (Variables|Default|GetIsDead))
    (Utilities|FlowControl|Sequence
      (:then_0
        (AI|AIMoveTo self "0, 0, 0" Pawn 5.0 false))
      (:then_1
        (Utilities|FlowControl|RetriggerableDelay 0.6)
        (CallFunction|Move)))
    (else
      (Components|Movement|StopMovementImmediately (Variables|Character|GetCharacterMovement)))))

(event Custom|Move
  ;[0 0 0] AI-Roam Logic
  (AI|AIMoveTo self (.RandomLocation (AI|Navigation|GetRandomReachablePointinRadius (Transformation|GetActorLocation) 5e+03 0 0)) 0 5.0 false
    (:OnSuccess
      (Utilities|FlowControl|Delay 3.0)
      (CallFunction|Move))))

(event EventTick
  (params (DeltaSeconds :type Float%20%28single-precision%29))
  ;[0 0 0] On Tick
  (CallFunction|TargetRangeCheck))

(event EventBeginPlay
  ;[0 0 0] Initialize
  (CallFunction|SetFirstPersonCharacter))

(event Game|Damage|EventAnyDamage
  (params (Damage :type Float%20%28single-precision%29) (DamageType :type Damage%20Type%20Object%20Reference) (InstigatedBy :type Controller%20Object%20Reference) (DamageCauser :type Actor%20Object%20Reference))
  ;[0 0 0] On Take Damage
  (Variables|Default|SetIsDead true)
  (Utilities|FlowControl|Delay 0.666)
  (CallFunction|SpawnUpgradeOrb)
  (Actor|DestroyActor))

(fn ConstructionScript)

(fn SpawnUpgradeOrb
  (Game|SpawnActorfromClass "/Game/EdgeOfSorrow/Blueprints/Collectibles/BP_UpgradeOrb.BP_UpgradeOrb_C" (Transformation|GetActorTransform) "Undefined" "MultiplyWithRoot" 0 0))

(fn SetFirstPersonCharacter
  (bind _returnvalue (Game|GetPlayerCharacter 0))
  (bind _asbp_first_person_character (Utilities|Casting|CastToBP_FirstPersonCharacter _returnvalue))
  (Utilities|IsValid _asbp_first_person_character
    (:Is%20Valid
      (Variables|Default|SetAs%20BP%20First%20Person%20Character _asbp_first_person_character))))

(fn TargetRangeCheck
  (bind _as_bp_first_person_character (Variables|Default|GetAs%20BP%20First%20Person%20Character))
  (Utilities|IsValid _as_bp_first_person_character
    (:Is%20Valid
      (if (<= (Transformation|GetDistanceTo _as_bp_first_person_character self) (Variables|Default|GetAttackDistance))
        (Variables|Default|SetIsTargetInRange true)))))