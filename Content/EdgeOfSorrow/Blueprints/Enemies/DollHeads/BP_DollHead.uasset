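; BP_DollHead is a doll head enemy that laughs like a toddler and damages actors that hit its capsule.
; BeginPlay runs parent setup, starts the laugh on a runtime-added audio component, and rotates the head mesh through the HeadBobbing timeline.
; Incoming damage updates health; at zero it stops the laugh, signals enemy destruction and runs death logic.
; SetSoundCue allows the laugh sound to be swapped.
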(event OnComponentHit(CapsuleComponent)
  (params (HitComponent :type Primitive%20Component%20Object%20Reference) (OtherActor :type Actor%20Object%20Reference) (OtherComp :type Primitive%20Component%20Object%20Reference) (NormalImpulse :type Vector :default "0, 0, 0") (Hit :type Hit%20Result%20Structure%20%28by%20ref%29))
  ;[0 0 0] Do Damage
  (CallFunction|DoDamage OtherActor))

(event EventBeginPlay
  (|CallParentFunction)
  (Utilities|FlowControl|Sequence
    (:then_0
      (bind _returnvalue (AddComponent|AddAudioComponent false))
      (bind _output_get (Variables|Default|SetToddlerLaugh _returnvalue))
      (Audio|Components|Audio|SetSound _output_get "/Game/EdgeOfSorrow/Audio/freesound_org/Enemies/SW_Toddler15MonthsLaugh_Cue.SW_Toddler15MonthsLaugh_Cue")
      (Audio|Components|Audio|Play (Variables|Default|GetToddlerLaugh) 0.0))
    (:then_1
      (bind _rotate (Timeline|HeadBobbing Play)
        (:Update
          (Transformation|AddLocalRotation (Variables|Default|GetSM_DollHead03) (Math|Rotator|MakeRotator _rotate _rotate _rotate) false false))))))

(event Game|Damage|EventAnyDamage
  (params (Damage :type Float%20%28single-precision%29) (DamageType :type Damage%20Type%20Object%20Reference) (InstigatedBy :type Controller%20Object%20Reference) (DamageCauser :type Actor%20Object%20Reference))
  (bind _toddlerlaugh (Variables|Default|GetToddlerLaugh))
  ;[0 0 0] On Take Damage
  (bind _health (CallFunction|UpdateHealth Damage))
  (if (<= _health 0.0)
    (Utilities|IsValid _toddlerlaugh
      (:Is%20Valid
        (Audio|Components|Audio|Stop _toddlerlaugh))
      (:Is%20Not%20Valid
        _))
    (Default|CallOnEnemyDestroyed)
    (CallFunction|OnDeath)))

(fn ConstructionScript)

(fn SetSoundCue
  (params (NewSoundCue :type Sound%20Cue%20Object%20Reference))
  (Audio|Components|Audio|SetSound (Variables|Default|GetToddlerLaugh) NewSoundCue))