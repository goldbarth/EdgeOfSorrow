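; Destructible doll head spawner that spawns enemies from a class queue at its spawn point.
; A looping timer drains the queue, and newly queued classes trigger an immediate spawn unless a doll head overlaps the capsule.
; It binds to each spawned enemy's destroyed event and has a handler that reports defeats to the arena game mode.
; A timeline pulses its material color, and damage depletes its health until it is destroyed.
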(event Custom|OnEnemyDefeated
  (bind _returnvalue (Game|GetGameMode))
  (bind _asbp_arena_game_mode (Utilities|Casting|CastToBP_ArenaGameMode _returnvalue))
  ;[0 0 0] Update the Enemy Queue
  (Utilities|IsValid _asbp_arena_game_mode
    (:Is%20Valid
      (Default|OnEnemyDefeated _asbp_arena_game_mode))))

(event Custom|TryToSpawn
  ;[0 0 0] Spawn loop
  (CallFunction|SpawnEnemy))

(event EventBeginPlay
  (Utilities|FlowControl|Sequence
    (:then_0
      (CallFunction|SetAudioComponent))
    (:then_1
      (bind _colorgradient (Timeline|PulsingEffect Play)
        (:Update
          (CallFunction|SetMaterialColor _colorgradient))))
    (:then_2
      ;[0 0 0] Spawn loop
      (Utilities|FlowControl|Delay 2.1)
      (Utilities|Time|SetTimerbyEvent (delegate Custom|TryToSpawn) 3.0 true))))

(event Game|Damage|EventAnyDamage
  (params (Damage :type Float%20%28single-precision%29) (DamageType :type Damage%20Type%20Object%20Reference) (InstigatedBy :type Controller%20Object%20Reference) (DamageCauser :type Actor%20Object%20Reference))
  (bind _dronesound (Variables|Default|GetDroneSound))
  ;[0 0 0] Take Damage
  (bind _isdestroyed (CallFunction|TakeDamage Damage))
  (if _isdestroyed
    (Actor|DestroyActor)
    (Utilities|IsValid _dronesound
      (:Is%20Valid
        (Audio|Components|Audio|Stop _dronesound)))))

(fn ConstructionScript)

(fn SpawnEnemy
  (if (Utilities|Array|IsValidIndex (Variables|Default|GetEnemyQueue))
    (bind _returnvalue (Game|SpawnActorfromClass (Utilities|Array|Get(acopy) (Variables|Default|GetEnemyQueue)) (Transformation|GetWorldTransform (Variables|Default|GetSpawnLocation)) "AdjustIfPossibleButAlwaysSpawn" "MultiplyWithRoot" 0 0))
    (Utilities|IsValid _returnvalue
      (:Is%20Valid
        (EventDispatchers|BindEventtoOnEnemyDestroyed _returnvalue (EventDispatchers|CreateEvent :!event Custom|OnEnemyDefeated))
        (Utilities|Array|RemoveIndex (Variables|Default|GetEnemyQueue))
        (return true)))
    (else
      (return false))))

(fn AddEnemytoQueue
  (params (EnemyClass :type BP%20Doll%20Head%20Class%20Reference%20%28by%20ref%29))
  (Utilities|Array|Add (Variables|Default|GetEnemyQueue) EnemyClass)
  (if (not (Utilities|Array|IsValidIndex (Collision|GetOverlappingActors (Variables|Default|GetCapsuleCollision) "/Game/EdgeOfSorrow/Blueprints/Enemies/DollHeads/BP_DollHead.BP_DollHead_C" :!class /Script/Engine.PrimitiveComponent)))
    (CallFunction|SpawnEnemy)))

(fn TakeDamage
  (params (Damage :type Float%20%28double-precision%29))
  (Variables|Default|SetHealth_0 (Math|Float|Truncate (- (Variables|Default|GetHealth_0) Damage)))
  (return (<= (Variables|Default|GetHealth_0) 0)))

(fn SetAudioComponent
  (bind _returnvalue (AddComponent|AddAudioComponent false))
  (Variables|Default|SetDroneSound _returnvalue))

(fn SetMaterialColor
  (params (InputPin :type Linear%20Color%20Structure))
  (bind _returnvalue (Rendering|Material|CreateDynamicMaterialInstance (Variables|Default|GetSM_Cave01) 0 "/Game/EdgeOfSorrow/Objects/Enemies/MI_DollHeadSpawner_Inst.MI_DollHeadSpawner_Inst" "None" :!class /Script/Engine.PrimitiveComponent))
  (Rendering|Material|SetVectorParameterValue _returnvalue (Variables|Default|GetParameter%20Name) InputPin :!class /Script/Engine.MaterialInstanceDynamic))