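; Exoskeleton gear that gives the first-person player a dash and adds its own HUD widget at BeginPlay.
; StartAction dashes only from the ground, launching the character along horizontal velocity scaled by a multiplier, with whoosh sound and camera shake.
; A counter compared against DashCooldown gates the launch, then resets after a Delay whose duration comes from the dash check.
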(event Custom|StartAction
  (bind _cooldowntime (CallFunction|Dash))
  (Utilities|FlowControl|Delay _cooldowntime)
  (Variables|Default|SetDashCooldownCounter 0))

(event EventBeginPlay
  (Utilities|FlowControl|Sequence
    (:then_0
      (CallFunction|SetFirstPersonCharacter))
    (:then_1
      (CallFunction|AddWidgettoViewpoert))))

(fn ConstructionScript)

(fn PerformDash
  (bind _firstpersoncharacter (Variables|Default|GetFirstPersonCharacter))
  (bind _returnvalue (Transformation|GetActorLocation _firstpersoncharacter))
  (bind _returnvalue_2 (Transformation|GetVelocity _firstpersoncharacter))
  (bind _iscooldownactive (CallFunction|IsCooldownActive))
  (if _iscooldownactive
    (Audio|PlaySoundatLocation "/Game/EdgeOfSorrow/Audio/freesound_org/706678__sadiquecat__whoosh-bamboo-3.706678__sadiquecat__whoosh-bamboo-3" _returnvalue "0, 0, 0" 1.0 1.0 0.0 0 0 0 0)
    (Camera|PlayWorldCameraShake "/Game/EdgeOfSorrow/Blueprints/Player/BP_CameraShake.BP_CameraShake_C" _returnvalue 0.0 3e+03)
    (Character|LaunchCharacter (Variables|Default|GetFirstPersonCharacter) (* (Math|Vector|MakeVector (.x _returnvalue_2) (.y _returnvalue_2) 0.0) (Variables|Default|GetDash%20Velocity%20Multiplyer)) false false)
    (bind _result (Math|Integer|IncrementInt (Variables|Default|GetDashCooldownCounter))
      (:%20%20
        _)))
  (return (== _result (Variables|Default|GetDashCooldown))))

(fn CheckifCanDash
  (params (CanDash :type Boolean))
  (if CanDash
    (if (AI|Components|NavMovement|IsFalling (Variables|/Script/Engine.Character|GetCharacterMovement (Variables|Default|GetFirstPersonCharacter)))
      (return (Math|Conversions|ToFloat(Integer) (Variables|Default|GetDashCooldown))))
    (else
      (return (Math|Conversions|ToFloat(Integer) (Variables|Default|GetDashCooldown))))))

(fn IsCooldownActive
  (return (!= (Variables|Default|GetDashCooldownCounter) (Variables|Default|GetDashCooldown))))

(fn SetFirstPersonCharacter
  (bind _returnvalue (Game|GetPlayerCharacter 0))
  (bind _asbp_first_person_character (Utilities|Casting|CastToBP_FirstPersonCharacter _returnvalue))
  (Utilities|IsValid _asbp_first_person_character
    (:Is%20Valid
      (Variables|Default|SetFirstPersonCharacter _asbp_first_person_character))))

(fn Dash
  (if (AI|Components|NavMovement|IsMovingonGround (Variables|/Script/Engine.Character|GetCharacterMovement (Variables|Default|GetFirstPersonCharacter)))
    (bind _iscooldown (CallFunction|PerformDash))
    (bind _cooldowntime (CallFunction|CheckifCanDash _iscooldown)))
  (return _cooldowntime))

(fn AddWidgettoViewpoert
  (bind _returnvalue (UserInterface|CreateWidget "/Game/EdgeOfSorrow/Blueprints/UI/HUD/WB_ExoskeletonHUD.WB_ExoskeletonHUD_C"))
  (bind _output_get (Variables|Default|SetExoskeletonHUD _returnvalue))
  (UserInterface|Viewport|AddtoViewport _output_get (Variables|Default|GetZOrderExoskeletonHUD)))