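; Force shield gear actor that drains the first-person character's shield power when its sphere is overlapped by tagged actors.
; On BeginPlay it caches the player character and adds a HUD widget with a material-driven indicator.
; A hit recolors the indicator and sets a cooldown flag; overlaps during cooldown instead start a named-function timer, presumably to clear it.
; When an overlap ends, the indicator restores its default look after a short delay.
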(event OnComponentBeginOverlap(SphereCollision)
  (params (OverlappedComponent :type Primitive%20Component%20Object%20Reference) (OtherActor :type Actor%20Object%20Reference) (OtherComp :type Primitive%20Component%20Object%20Reference) (OtherBodyIndex :type Integer) (bFromSweep :type Boolean) (SweepResult :type Hit%20Result%20Structure%20%28by%20ref%29))
  (CallFunction|TryGetHit OtherActor))

(event OnComponentEndOverlap(SphereCollision)
  (params (OverlappedComponent :type Primitive%20Component%20Object%20Reference) (OtherActor :type Actor%20Object%20Reference) (OtherComp :type Primitive%20Component%20Object%20Reference) (OtherBodyIndex :type Integer))
  (Utilities|FlowControl|Delay 0.2)
  (CallFunction|ChangeMaterialParameter "(R=0.024572,G=1.288960,B=2.000000,A=1.000000)" 1.2 3.0))

(event EventBeginPlay
  (Utilities|FlowControl|Sequence
    (:then_0
      (CallFunction|SetFirstPersonCharacter))
    (:then_1
      (CallFunction|CreateWidget))))

(fn ConstructionScript)

(fn ChangeMaterialParameter
  (params (IndicatorColor :type Linear%20Color%20Structure) (IndicatorStrenght :type Float%20%28double-precision%29) (Opacity :type Float%20%28double-precision%29))
  (bind _forceshieldhud (Variables|Default|GetForceShieldHUD))
  (bind _indicator (Variables|/Game/EdgeOfSorrow/Blueprints/UI/HUD/WB_ForceShieldHUD.WB_ForceShieldHUD_C|GetIndicator _forceshieldhud))
  (bind _brush (Variables|/Script/UMG.Image|GetBrush _indicator))
  (bind _returnvalue (Appearance|GetDynamicMaterial _brush :!class /Script/UMG.WidgetBlueprintLibrary))
  (Rendering|Material|SetVectorParameterValue _returnvalue (Variables|Default|GetBaseColorParameter) IndicatorColor :!class /Script/Engine.MaterialInstanceDynamic)
  (Rendering|Material|SetScalarParameterValue _returnvalue (Variables|Default|GetIndicatorStrenghtParameter) IndicatorStrenght :!class /Script/Engine.MaterialInstanceDynamic)
  (Rendering|Material|SetScalarParameterValue _returnvalue (Variables|Default|GetOpacityParameter) Opacity :!class /Script/Engine.MaterialInstanceDynamic))

(fn ResetCooldown
  (Variables|Default|SetIsCooldown false))

(fn GetHit
  (params (IndicatorColor :type Linear%20Color%20Structure :default "(R=0.672443,G=0.000000,B=0.644480,A=1.000000)") (IndicatorStrenght :type Float%20%28double-precision%29) (Opacity :type Float%20%28double-precision%29))
  (Variables|Default|SetIsCooldown true)
  (CallFunction|ChangeMaterialParameter IndicatorColor IndicatorStrenght Opacity)
  (Default|DecreaseShieldPower (Variables|Default|GetFirstPersonCharacter)))

(fn TryGetHit
  (params (OtherActor :type Actor%20Object%20Reference))
  (if (Actor|ActorHasTag OtherActor (Variables|Default|GetOtherActorTag))
    (if (Variables|Default|GetIsCooldown)
      (Utilities|Time|SetTimerbyFunctionName 0 (Variables|Default|GetFunction%20Name) (Variables|Default|GetCooldownTime))
      (else
        (CallFunction|GetHit (Variables|Default|GetHitIndicatorColor) (Variables|Default|GetHitIndicatorStrength) (Variables|Default|GetHitOpacity))))))

(fn SetFirstPersonCharacter
  (Variables|Default|SetFirstPersonCharacter (.AsBP%20First%20Person%20Character (Utilities|Casting|CastToBP_FirstPersonCharacter (Game|GetPlayerCharacter 0)))))

(fn CreateWidget
  (bind _returnvalue (UserInterface|CreateWidget "/Game/EdgeOfSorrow/Blueprints/UI/HUD/WB_ForceShieldHUD.WB_ForceShieldHUD_C"))
  (bind _output_get (Variables|Default|SetForceShieldHUD _returnvalue))
  (UserInterface|Viewport|AddtoViewport _output_get -10))