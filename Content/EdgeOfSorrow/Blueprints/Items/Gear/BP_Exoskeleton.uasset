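; Exoskeleton gear item that gives the first-person player character a ground dash with a cooldown.
; ExoskeletonDash launches the character along its horizontal velocity scaled by a multiplier, with a whoosh sound and camera shake.
; A counter blocks dashes once it equals DashCooldown, and a Delay timed by the dash check's result resets it.
; Despite its name, IsCooldownActive returns true while dashing is still allowed.
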(event Custom|ExoskeletonDash
  (bind _cooldowntime (CallFunction|Dash))
  (Utilities|FlowControl|Delay _cooldowntime)
  (Variables|Default|SetDashCooldownCounter 0))

(event EventBeginPlay
  (CallFunction|SetFirstPersonCharacter))

(fn ConstructionScript)

(fn PerformDash
  (bind _as_bp_first_person_character (Variables|Default|GetAs%20BP%20First%20Person%20Character))
  (bind _returnvalue (Transformation|GetActorLocation _as_bp_first_person_character))
  (bind _returnvalue_2 (Transformation|GetVelocity _as_bp_first_person_character))
  (bind _iscooldownactive (CallFunction|IsCooldownActive))
  (if _iscooldownactive
    (Audio|PlaySoundatLocation "/Game/EdgeOfSorrow/Audio/freesound_org/706678__sadiquecat__whoosh-bamboo-3.706678__sadiquecat__whoosh-bamboo-3" _returnvalue "0, 0, 0" 1.0 1.0 0.0 0 0 0 0)
    (Camera|PlayWorldCameraShake "/Game/EdgeOfSorrow/Blueprints/Player/Movement/BP_CameraShakeRightDash.BP_CameraShakeRightDash_C" _returnvalue 0.0 3e+03)
    (Character|LaunchCharacter (Variables|Default|GetAs%20BP%20First%20Person%20Character) (* (Math|Vector|MakeVector (.x _returnvalue_2) (.y _returnvalue_2) 0.0) (Variables|Default|GetDash%20Velocity%20Multiplyer)) false false)
    (bind _result (Math|Integer|IncrementInt (Variables|Default|GetDashCooldownCounter))
      (:%20%20
        _)))
  (return (== _result (Variables|Default|GetDashCooldown))))

(fn CheckifCanDash
  (params (CanDash :type Boolean))
  (if CanDash
    (if (AI|Components|NavMovement|IsFalling (Variables|/Script/Engine.Character|GetCharacterMovement (Variables|Default|GetAs%20BP%20First%20Person%20Character)))
      (return (Math|Conversions|ToFloat(Integer) (Variables|Default|GetDashCooldown))))
    (else
      (return (Math|Conversions|ToFloat(Integer) (Variables|Default|GetDashCooldown))))))

(fn IsCooldownActive
  (return (!= (Variables|Default|GetDashCooldownCounter) (Variables|Default|GetDashCooldown))))

(fn SetFirstPersonCharacter
  (bind _returnvalue (Game|GetPlayerCharacter 0))
  (bind _asbp_first_person_character (Utilities|Casting|CastToBP_FirstPersonCharacter _returnvalue))
  (Utilities|IsValid _asbp_first_person_character
    (:Is%20Valid
      (Variables|Default|SetAs%20BP%20First%20Person%20Character _asbp_first_person_character))))

(fn Dash
  (if (AI|Components|NavMovement|IsMovingonGround (Variables|/Script/Engine.Character|GetCharacterMovement (Variables|Default|GetAs%20BP%20First%20Person%20Character)))
    (bind _iscooldown (CallFunction|PerformDash))
    (bind _cooldowntime (CallFunction|CheckifCanDash _iscooldown)))
  (return _cooldowntime))