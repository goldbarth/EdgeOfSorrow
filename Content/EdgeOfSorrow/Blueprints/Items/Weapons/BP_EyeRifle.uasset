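; BP_EyeRifle is a full-auto rifle that fires eye-rifle projectiles with a shot sound and first-person montage.
; StartAction passes a cooldown check, then starts a looping timer at the game instance's FireRate, using a negative start delay to fire immediately.
; StopAction clears the timer, and OnUpdateFireRate restarts it mid-burst to apply a changed rate.
; IsCooldownActive returns true once the cooldown has elapsed, despite its name.
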(event Custom|OnFireProjectile
  ;[0 0 0] Full-Auto
  (CallFunction|SpawnProjectile "/Game/EdgeOfSorrow/Blueprints/Projectiles/BP_EyeRifleProjectile.BP_EyeRifleProjectile_C" "/Game/EdgeOfSorrow/Audio/GDC_GameAudio/SW_HeavyweaponShot.SW_HeavyweaponShot" "/Game/EdgeOfSorrow/Character/Animations/FP_Rifle_Shoot_Montage.FP_Rifle_Shoot_Montage"))

(event Custom|OnUpdateFireRate
  (bind _gameinstance (Variables|Default|GetGameInstance))
  (bind _firerate (Variables|/Game/EdgeOfSorrow/Blueprints/BP_GameInstance.BP_GameInstance_C|GetFireRate _gameinstance))
  ;[0 0 0] Full-Auto
  (Utilities|Time|ClearandInvalidateTimerbyHandle (stale _returnvalue))
  (if (Variables|Default|GetIsActionOngoing)
    (bind _returnvalue (Utilities|Time|SetTimerbyEvent (delegate Custom|OnFireProjectile) _firerate true (* _firerate -1.0)))))

(event EventBeginPlay
  (CallFunction|SetGameInstance))

(event EventStartAction
  (bind _gameinstance (Variables|Default|GetGameInstance))
  (bind _firerate (Variables|/Game/EdgeOfSorrow/Blueprints/BP_GameInstance.BP_GameInstance_C|GetFireRate _gameinstance))
  ;[0 0 0] Full-Auto
  (Variables|Default|SetIsActionOngoing true)
  (bind _returnvalue (CallFunction|IsCooldownActive))
  (if _returnvalue
    (Variables|Default|SetLastFireTime (Utilities|Time|GetGameTimeinSeconds))
    (bind _returnvalue_2 (Utilities|Time|SetTimerbyEvent (delegate Custom|OnFireProjectile) _firerate true (* _firerate -1.0)))))

(event EventStopAction
  (bind _gameinstance (Variables|Default|GetGameInstance))
  (bind _firerate (Variables|/Game/EdgeOfSorrow/Blueprints/BP_GameInstance.BP_GameInstance_C|GetFireRate _gameinstance))
  ;[0 0 0] Full-Auto
  (Variables|Default|SetIsActionOngoing false)
  (Utilities|Time|ClearandInvalidateTimerbyHandle (stale _returnvalue))
  (if (Variables|Default|GetIsActionOngoing)
    (bind _returnvalue (Utilities|Time|SetTimerbyEvent (delegate Custom|OnFireProjectile) _firerate true (* _firerate -1.0)))))

(fn ConstructionScript)

(fn IsCooldownActive
  (return (>= (- (Utilities|Time|GetGameTimeinSeconds) (Variables|Default|GetLastFireTime)) (Variables|/Game/EdgeOfSorrow/Blueprints/BP_GameInstance.BP_GameInstance_C|GetFireRate (Variables|Default|GetGameInstance)))))

(fn SetGameInstance
  (Variables|Default|SetGameInstance (.AsBP%20Game%20Instance (Utilities|Casting|CastToBP_GameInstance (Game|GetGameInstance)))))