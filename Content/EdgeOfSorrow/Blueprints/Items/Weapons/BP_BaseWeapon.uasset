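; BP_BaseWeapon is a base weapon that fires projectiles toward the player's crosshair, with empty start, stop and fire-rate events.
; SpawnProjectile spawns at an arrow component, plays the fire sound and triggers the first-person character's shoot montage.
; Aim comes from deprojecting the offset crosshair and tracing on Visibility.
; The projectile rotates toward the trace's hit location, which is used without checking for a hit.
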(event Custom|OnUpdateFireRate)

(event EventBeginPlay
  (CallFunction|SetFirstPersonCharacter))

(event EventStartAction)

(event EventStopAction)

(fn ConstructionScript)

(fn SpawnProjectile
  (params (ProjectileType :type Actor%20Class%20Reference) (FireSound :type Sound%20Base%20Object%20Reference) (MontageToPlay :type Anim%20Montage%20Object%20Reference))
  (bind _returnvalue (Game|GetPlayerCharacter 0))
  (bind _spawnlocationarrow (Variables|Default|GetSpawnLocationArrow))
  (bind _asbp_first_person_character (Utilities|Casting|CastToBP_FirstPersonCharacter _returnvalue))
  (LocalVariables|SetSpawnLocation (Transformation|GetWorldLocation _spawnlocationarrow))
  (bind _hitlocation (CallFunction|EvaluateProjectileDirection))
  (bind _returnvalue_2 (Game|SpawnActorfromClass ProjectileType (Transformation|GetWorldTransform _spawnlocationarrow) "Undefined" "MultiplyWithRoot" 0 0))
  (Transformation|SetActorRotation _returnvalue_2 (Math|Rotator|FindLookatRotation (LocalVariables|GetSpawnLocation) _hitlocation))
  (Audio|PlaySoundatLocation FireSound (LocalVariables|GetSpawnLocation) "0, 0, 0" 1.0 1.0 0.0 0 0 0 0)
  (Utilities|IsValid _asbp_first_person_character
    (:Is%20Valid
      (Default|PlayShootAnimation _asbp_first_person_character MontageToPlay))))

(fn SetFirstPersonCharacter
  (bind _returnvalue (Game|GetPlayerCharacter 0))
  (bind _asbp_first_person_character (Utilities|Casting|CastToBP_FirstPersonCharacter _returnvalue))
  (Utilities|IsValid _asbp_first_person_character
    (:Is%20Valid
      (Variables|Default|SetFirstPersonCharacter _asbp_first_person_character))))

(fn EvaluateProjectileDirection
  (bind (_start _end) (CallFunction|CalculateStartEndPosition))
  (bind _outhit (Collision|LineTraceByChannel _start _end "TraceTypeQuery1" false 0 "None" true "(R=0.000000,G=0.000000,B=0.000000,A=1.000000)" "(R=0.000000,G=0.000000,B=0.000000,A=1.000000)"))
  (bind _output_get (Variables|Default|SetHitLocation (.Location (Collision|BreakHitResult _outhit))))
  (return _output_get))

(fn CalculateStartEndPosition
  (bind _returnvalue (Viewport|GetViewportSize))
  (bind _returnvalue_2 (Game|GetPlayerController 0))
  (bind _divideviewport (Variables|Default|GetDivideViewport))
  (bind _crosshairoffset (Variables|Default|GetCrosshairOffset))
  (bind _returnvalue_3 (/ _returnvalue _divideviewport))
  (bind _returnvalue_4 (+ _returnvalue_3 (Math|Vector2D|MakeVector2D 0.0 _crosshairoffset)))
  (bind (_worldposition _worlddirection) (Class|GameplayStatics|DeprojectScreentoWorld _returnvalue_2 _returnvalue_4))
  (return _worldposition (+ (* _worlddirection (Variables|Default|GetProjectileDistance)) (Camera|GetCameraLocation (Game|GetPlayerCameraManager 0)))))