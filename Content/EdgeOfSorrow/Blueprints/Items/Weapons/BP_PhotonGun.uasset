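; BP_PhotonGun is a charge-and-release beam weapon that damages whatever its line trace hits.
; StartAction plays a charging sound and applies charge settings to the Niagara beam through SetPhotonBeamValues.
; StopAction applies release settings with an endpoint from the trace end's X, plays the release sound, calls HitEnemy, then zeroes the beam after a short delay.
; Tick calls a debug helper whose trace and print are disconnected.
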(event Custom|ResetPhotonBeamToZero
  (Utilities|FlowControl|Delay 0.5)
  (CallFunction|SetPhotonBeamValues "0, 0, 0" 0.0 0.0 0.0))

(event EventTick
  (params (DeltaSeconds :type Float%20%28single-precision%29))
  (CallFunction|DEBUGHitActorLineTrace))

(event EventStopAction
  (CallFunction|ReleasePhotonBeam))

(event EventStartAction
  (CallFunction|ChargePhotonBeam))

(fn ConstructionScript)

(fn ChargePhotonBeam
  (bind _returnvalue (Audio|SpawnSound2D (Variables|Default|GetChargingSound) 1.0 1.0 0.0 0))
  (Variables|Default|SetChargingSoundComponent _returnvalue)
  (CallFunction|SetPhotonBeamValues (Variables|Default|GetChargeEndPoint) (Variables|Default|GetChargeBeamWidth) (Variables|Default|GetChargeNoiseFrequency) (Variables|Default|GetChargeNoiseCurve)))

(fn ReleasePhotonBeam
  (bind _chargingsoundcomponent (Variables|Default|GetChargingSoundComponent))
  (Utilities|IsValid _chargingsoundcomponent
    (:Is%20Valid
      (Audio|Components|Audio|Stop _chargingsoundcomponent)
      (bind _end (CallFunction|CalculateStartEndPosition))
      (bind _output_get (LocalVariables|SetEndX (.x _end)))
      (if (<= _output_get 1e+02)
        (LocalVariables|SetEndX 1e+03)))
    (:Is%20Not%20Valid
      _))
  (CallFunction|SetPhotonBeamValues (Math|Vector|MakeVector (LocalVariables|GetEndX) 0.0 0.0) (Variables|Default|GetReleaseBeamWidth) (Variables|Default|GetReleaseNoiseFrequency) (Variables|Default|GetReleaseNoiseCurve))
  (Audio|SpawnSound2D (Variables|Default|GetReleaseSound) 1.0 1.0 0.0 0)
  (CallFunction|HitEnemy "None")
  (CallFunction|ResetPhotonBeamtoZero))

(fn SetPhotonBeamValues
  (params (EndPoint :type Vector) (Width :type Float%20%28double-precision%29) (NoiseFrequency :type Float%20%28double-precision%29) (NoiseCurve :type Float%20%28double-precision%29))
  (bind _ns_photonbeam (Variables|Default|GetNS_PhotonBeam))
  (Niagara|SetNiagaraVariable(Vector3) _ns_photonbeam "BeamEndpoint" EndPoint)
  (Niagara|SetNiagaraVariable(Float) _ns_photonbeam "BeamWidth" Width)
  (Niagara|SetNiagaraVariable(Float) _ns_photonbeam "NoiseFrequency" NoiseFrequency)
  (Niagara|SetNiagaraVariable(Float) _ns_photonbeam "NoiseCurve" NoiseCurve))

(fn HitEnemy
  (params (DrawDebugType :type EDrawDebugTrace%20Enum :default "None"))
  (bind (_start _end) (CallFunction|CalculateStartEndPosition))
  (bind _outhit (Collision|LineTraceByChannel _start _end "TraceTypeQuery1" false 0 DrawDebugType true "(R=0.000000,G=0.000000,B=0.000000,A=1.000000)" "(R=0.000000,G=0.000000,B=0.000000,A=1.000000)"))
  (Game|Damage|ApplyDamage (.HitActor (Collision|BreakHitResult _outhit)) (Variables|Default|GetBase%20Damage) 0 0))

(fn DEBUGHitActorLineTrace
  (bind (_start _end) (CallFunction|CalculateStartEndPosition)))