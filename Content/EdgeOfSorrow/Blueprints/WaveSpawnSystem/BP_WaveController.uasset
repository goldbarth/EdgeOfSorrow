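; BP_WaveController runs enemy waves, spawning a BP_Charger at every BP_SpawnPoint each wave.
; Tick polls for actors tagged "Enemy" and calls NewWave when none remain, which increments WaveCount until it reaches WaveAmount.
; SetGameMode caches the arena game mode but is not called here, and the SpawnExit call is disconnected, so finishing the last wave triggers nothing.
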(event EventTick
  (params (DeltaSeconds :type Float%20%28single-precision%29))
  (bind _outactors (Actor|GetAllActorswithTag "Enemy"))
  (if (<= (Utilities|Array|Length _outactors) 0)
    (CallFunction|NewWave)))

(event EventBeginPlay)

(fn ConstructionScript)

(fn NewWave
  (if (not (>= (Variables|Default|GetWaveCount) (Variables|Default|GetWaveAmount)))
    (Math|Integer|IncrementInt (Variables|Default|GetWaveCount)
      (:%20%20
        (bind _outactors (Actor|GetAllActorsOfClass "/Game/EdgeOfSorrow/Blueprints/WaveSpawnSystem/BP_SpawnPoint.BP_SpawnPoint_C"))
        (for _array_element _outactors
          (Game|SpawnActorfromClass "/Game/EdgeOfSorrow/Blueprints/Enemies/BP_Charger.BP_Charger_C" (Transformation|GetActorTransform _array_element) "Undefined" "MultiplyWithRoot" 0 0))))))

(fn SetGameMode
  (bind _returnvalue (Game|GetGameMode))
  (bind _asbp_arena_game_mode (Utilities|Casting|CastToBP_ArenaGameMode _returnvalue))
  (Utilities|IsValid _asbp_arena_game_mode
    (:Is%20Valid
      (Variables|Default|SetArenaGameMode _asbp_arena_game_mode))))