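; BP_DepthChangeObject is an environment object that reacts when a round is won in the arena.
; On BeginPlay it gets and caches the BP_ArenaGameMode, then binds to its OnRoundWon event.
; The handler only calls OnRoundWonMessage, which has no implementation here, so this Blueprint itself defines no depth-change behavior.
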(event Custom|RoundWon
  (Class|INotificationDispatcher|OnRoundWon(Message) self))

(event EventBeginPlay
  (bind _gamemode (CallFunction|SetArenaGameMode))
  (EventDispatchers|BindEventtoOnRoundWon _gamemode (delegate Custom|RoundWon)))

(fn ConstructionScript)

(fn SetArenaGameMode
  (bind _returnvalue (Game|GetGameMode))
  (bind _asbp_arena_game_mode (Utilities|Casting|CastToBP_ArenaGameMode _returnvalue))
  (Utilities|IsValid _asbp_arena_game_mode
    (:Is%20Valid
      (bind _output_get (Variables|Default|SetArenaGameMode _asbp_arena_game_mode))
      (return _output_get))))