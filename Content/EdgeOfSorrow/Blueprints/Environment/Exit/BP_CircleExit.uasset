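; BP_CircleExit is a level exit that ends the level when an actor tagged Player hits its box collision.
; StartWinFeedback plays a sound, stops the first-person character, disables movement and input, brightens and tints the rect light, and swaps the ruins circle's materials.
; After a short delay it opens the level named by LevelName.
; Other actors only trigger a joke debug print, and OnRoundWon is an empty stub.
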(event OnComponentHit(BoxCollision)
  (params (HitComponent :type Primitive%20Component%20Object%20Reference) (OtherActor :type Actor%20Object%20Reference) (OtherComp :type Primitive%20Component%20Object%20Reference) (NormalImpulse :type Vector :default "0, 0, 0") (Hit :type Hit%20Result%20Structure%20%28by%20ref%29))
  (Utilities|IsValid OtherActor
    (:Is%20Valid
      (if (not (Actor|ActorHasTag OtherActor "Player"))
        (Development|PrintString "NICE TRY PASCAL :P" true true "(R=0.000000,G=1.000000,B=0.056510,A=1.000000)" 1e+01) ; I need Sleep :)
        (else
          (CallFunction|StartWinFeedback)
          (Utilities|FlowControl|Delay 2.0)
          (Game|OpenLevel(byName) (Variables|Default|GetLevel%20Name)))))))

(event EventOnRoundWon)

(fn ConstructionScript)

(fn SetMaterials
  (params (Mesh :type Static%20Mesh%20Component%20Object%20Reference) (Material :type Material%20Object%20Reference))
  (Rendering|Material|SetMaterial Mesh 0 Material)
  (Rendering|Material|SetMaterial Mesh 1 Material))

(fn StartWinFeedback
  (bind _returnvalue (Game|GetPlayerCharacter 0))
  (bind _returnvalue_2 (Game|GetPlayerController 0))
  (bind _rectlight (Variables|Default|GetRectLight))
  (bind _asbp_first_person_character (Utilities|Casting|CastToBP_FirstPersonCharacter _returnvalue))
  (bind _asbp_player_controller (Utilities|Casting|CastToBP_PlayerController _returnvalue_2))
  (bind _charactermovement (Variables|/Script/Engine.Character|GetCharacterMovement _asbp_first_person_character))
  (Audio|PlaySound2D "/Game/EdgeOfSorrow/Audio/GDC_GameAudio/SW_PassiveGainLifeSound_Cue.SW_PassiveGainLifeSound_Cue" 1.0 1.0 0.0 0 0)
  (Utilities|IsValid _asbp_first_person_character
    (:Is%20Valid
      (Variables|/Game/EdgeOfSorrow/Blueprints/Player/BP_FirstPersonCharacter.BP_FirstPersonCharacter_C|SetIsRunning _asbp_first_person_character false)
      (Variables|/Script/Engine.MovementComponent|SetVelocity _charactermovement (Math|Vector|VectorZero))
      (Pawn|Components|CharacterMovement|DisableMovement _charactermovement)
      (Utilities|IsValid _asbp_player_controller
        (:Is%20Valid
          (Input|DisableInput _asbp_player_controller 0)
          (Rendering|Components|Light|SetIntensity _rectlight 6e+04)
          (Rendering|Components|Light|SetLightColor _rectlight "(R=1.000000,G=0.844751,B=0.519815,A=1.000000)" true)
          (CallFunction|SetMaterials (Variables|Default|GetSM_RuinsCircle) "/Game/EdgeOfSorrow/Materials/CelColors/M_CelColor9.M_CelColor9"))))))