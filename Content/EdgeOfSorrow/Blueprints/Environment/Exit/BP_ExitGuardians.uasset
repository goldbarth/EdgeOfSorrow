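; BP_ExitGuardians is an environment Blueprint for the exit that reacts when an arena round is won.
; On BeginPlay it caches the arena game mode, binds to its OnRoundWon event and caches the first-person player character.
; When the round is won, it sets IsRoundWon and calls OnRoundWonMessage, whose behavior is not defined in these graphs.
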(event Custom|RoundWon
  ;[0 0 0] Initialize
  (Variables|Default|SetIsRoundWon true)
  (Class|INotificationDispatcher|OnRoundWon(Message) self))

(event EventBeginPlay
  ;[0 0 0] Initialize
  (Utilities|FlowControl|Sequence
    (:then_0
      (bind _gamemode (CallFunction|SetArenaGameMode))
      (EventDispatchers|BindEventtoOnRoundWon _gamemode (delegate Custom|RoundWon)))
    (:then_1
      (CallFunction|SetFirstPersonCharacter))))

(fn ConstructionScript)

(fn SetArenaGameMode
  (bind _returnvalue (Game|GetGameMode))
  (bind _asbp_arena_game_mode (Utilities|Casting|CastToBP_ArenaGameMode _returnvalue))
  (Utilities|IsValid _asbp_arena_game_mode
    (:Is%20Valid
      (bind _output_get (Variables|Default|SetArenaGameMode _asbp_arena_game_mode))
      (return _output_get))))

(fn SetFirstPersonCharacter
  (bind _returnvalue (Game|GetPlayerCharacter 0))
  (bind _asbp_first_person_character (Utilities|Casting|CastToBP_FirstPersonCharacter _returnvalue))
  (Utilities|IsValid _asbp_first_person_character
    (:Is%20Valid
      (Variables|Default|SetFirstPersonCharacter _asbp_first_person_character))))