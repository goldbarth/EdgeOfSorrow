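; BP_GiantSkull is a giant skull environment actor that reacts when the round is won.
; On the round-won event it enables custom depth rendering on its skull mesh.
; While the round-won flag is set, Tick rotates the whole actor each frame to face the first-person character, if that reference is valid.
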(event EventTick
  (params (DeltaSeconds :type Float%20%28single-precision%29))
  (bind _firstpersoncharacter (Variables|Default|GetFirstPersonCharacter))
  (if (Variables|Default|GetIsRoundWon)
    (Utilities|IsValid _firstpersoncharacter
      (:Is%20Valid
        (Transformation|SetActorRotation (Math|Rotator|FindLookatRotation (Transformation|GetActorLocation) (Transformation|GetActorLocation _firstpersoncharacter)))))))

(event EventOnRoundWon
  (CallFunction|SetCustomDepth))

(fn ConstructionScript)

(fn SetCustomDepth
  (Rendering|SetRenderCustomDepth (Variables|Default|GetSM_GiantSkull01) true))