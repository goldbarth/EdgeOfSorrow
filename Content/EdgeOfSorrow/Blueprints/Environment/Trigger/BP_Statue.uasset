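; BP_Statue is an arena statue that becomes vulnerable once no BP_Charger enemies remain, then ends the level to the Shop when hit.
; Every Tick it counts BP_Charger actors in the world, and at zero swaps the statue mesh material and sets a vulnerable flag.
; A hit on its collision capsule while vulnerable calls EndLevel on BP_ArenaGameMode.
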(event OnComponentHit(CollideCapsule)
  (params (HitComponent :type Primitive%20Component%20Object%20Reference) (OtherActor :type Actor%20Object%20Reference) (OtherComp :type Primitive%20Component%20Object%20Reference) (NormalImpulse :type Vector :default "0, 0, 0") (Hit :type Hit%20Result%20Structure%20%28by%20ref%29))
  (if (Variables|Default|GetIsVunerable)
    (Default|EndLevel (.AsBP%20Arena%20Game%20Mode (Utilities|Casting|CastToBP_ArenaGameMode (Game|GetGameMode))) "Shop")))

(event EventTick
  (params (DeltaSeconds :type Float%20%28single-precision%29))
  (bind _returnvalue (CallFunction|CheckEnemyCount "/Game/EdgeOfSorrow/Blueprints/Enemies/BP_Charger.BP_Charger_C"))
  (if _returnvalue
    (CallFunction|SetVulnerable)))

(fn ConstructionScript)

(fn CheckEnemyCount
  (params (ActorClass :type Actor%20Class%20Reference))
  (bind _outactors (Actor|GetAllActorsOfClass ActorClass))
  (return (<= (Utilities|Array|Length _outactors) 0)))

(fn SetVulnerable
  (Rendering|Material|SetMaterial (Variables|Default|GetSM_Statue03) 0 "/Game/EdgeOfSorrow/Materials/CelColors/M_CelColor7.M_CelColor7")
  (Variables|Default|SetIsVunerable true))