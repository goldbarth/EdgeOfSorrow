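; BP_SpawnableExitPortal is a spawnable exit portal that marks the exit's position and carries a randomly chosen guardian.
; On BeginPlay it writes its location to the ExitPosition parameter of MPC_DarknessCollection, so materials using that collection can read where the exit is.
; It then picks a random class from the Guardians array and assigns it to the Guardian child actor component.
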(event EventBeginPlay
  (Utilities|FlowControl|Sequence
    (:then_0
      (CallFunction|SetLightPositiontoExit))
    (:then_1
      (CallFunction|SetRandomGuardian))))

(fn ConstructionScript)

(fn SetLightPositiontoExit
  (Rendering|Material|SetVectorParameterValue "/Game/EdgeOfSorrow/PostProcessing/CelShading_Darkness/MPC_DarknessCollection.MPC_DarknessCollection" "ExitPosition" (Math|Conversions|ToLinearColor(Vector) (Transformation|GetActorLocation)) :!class /Script/Engine.KismetMaterialLibrary))

(fn SetRandomGuardian
  (bind _output_get (Variables|Default|SetRandomIndex (Math|Random|RandomIntegerinRange 0 (- (Utilities|Array|Length (Variables|Default|GetGuardians)) 1))))
  (ChildActorComponent|SetChildActorClass (Variables|Default|GetGuardian) (Utilities|Array|Get(acopy) (Variables|Default|GetGuardians) _output_get)))