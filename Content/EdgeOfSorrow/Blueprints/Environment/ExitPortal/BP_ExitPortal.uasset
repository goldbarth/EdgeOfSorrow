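; Exit portal actor that ends a level when an actor tagged Player hits its box collision.
; Contact plays a sound, freezes the first-person character, and brightens and recolors the portal's light and ruins circle.
; After a short delay it checks the Game Instance's level index, either pausing with a win screen on the final level or opening the named level.
; Non-player hits only print a joke debug message.
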(event OnComponentHit(BoxCollision)
  (params (HitComponent :type Primitive%20Component%20Object%20Reference) (OtherActor :type Actor%20Object%20Reference) (OtherComp :type Primitive%20Component%20Object%20Reference) (NormalImpulse :type Vector :default "0, 0, 0") (Hit :type Hit%20Result%20Structure%20%28by%20ref%29))
  (Utilities|IsValid OtherActor
    (:Is%20Valid
      (if (not (Actor|ActorHasTag OtherActor "Player"))
        (Development|PrintString "NICE TRY PASCAL :P" true true "(R=0.000000,G=1.000000,B=0.056510,A=1.000000)" 1e+01) ; I need Sleep :)
        (else
          (CallFunction|StartWinFeedback)
          (Utilities|FlowControl|Delay 2.0)
          (if (== (Variables|/Game/EdgeOfSorrow/Blueprints/BP_GameInstance.BP_GameInstance_C|GetLevelIndex (Variables|Default|GetGameInstance)) 6)
            (Game|SetGamePaused true)
            (Viewport|RemoveAllWidgets)
            (bind _returnvalue (UserInterface|CreateWidget "/Game/EdgeOfSorrow/Blueprints/UI/Game/WB_WinScreen.WB_WinScreen_C"))
            (UserInterface|Viewport|AddtoViewport _returnvalue 0)
            (else
              (Game|OpenLevel(byName) (Variables|Default|GetLevel%20Name)))))))))

(event EventOnRoundWon)

(event EventBeginPlay
  (CallFunction|SetGameInstance))

(fn ConstructionScript)

(fn SetMaterials
  (params (Mesh :type Static%20Mesh%20Component%20Object%20Reference) (Material :type Material%20Object%20Reference))
  (Rendering|Material|SetMaterial Mesh 0 Material)
  (Rendering|Material|SetMaterial Mesh 1 Material))

(fn StartWinFeedback
  (bind _returnvalue (Game|GetPlayerCharacter 0))
  (bind _rectlight (Variables|Default|GetRectLight))
  (bind _asbp_first_person_character (Utilities|Casting|CastToBP_FirstPersonCharacter _returnvalue))
  (Audio|PlaySound2D "/Game/EdgeOfSorrow/Audio/GDC_GameAudio/SW_PassiveGainLifeSound_Cue.SW_PassiveGainLifeSound_Cue" 1.0 1.0 0.0 0 0)
  (Utilities|IsValid _asbp_first_person_character
    (:Is%20Valid
      (Default|FreezeMovementCompletely _asbp_first_person_character)
      (Input|DisableInput 0)
      (Rendering|Components|Light|SetIntensity _rectlight 6e+04)
      (Rendering|Components|Light|SetLightColor _rectlight "(R=1.000000,G=0.844751,B=0.519815,A=1.000000)" true)
      (CallFunction|SetMaterials (Variables|Default|GetSM_RuinsCircle) "/Game/EdgeOfSorrow/Materials/CelColors/M_CelColor9.M_CelColor9"))))

(fn SetGameInstance
  (bind _returnvalue (Game|GetGameInstance))
  (bind _asbp_game_instance (Utilities|Casting|CastToBP_GameInstance _returnvalue))
  (Utilities|IsValid _asbp_game_instance
    (:Is%20Valid
      (Variables|Default|SetGameInstance _asbp_game_instance))))