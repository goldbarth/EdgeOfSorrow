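; Photon gun weapon Blueprint that charges a beam on StartAction and fires it on StopAction.
; Charge and release each play a 2D sound and push their own endpoint, width and noise settings to a Niagara beam.
; Release also applies damage through a forward line trace from the spawn arrow, then resets the beam after a short delay.
; A debug trace draws and prints the aimed-at actor every Tick.
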(event Custom|ResetPhotonBeamToZero
  (Utilities|FlowControl|Delay 0.5)
  (CallFunction|SetPhotonBeamValues "0, 0, 0" 0.0 0.0 0.0))

(event EventTick
  (params (DeltaSeconds :type Float%20%28single-precision%29))
  (CallFunction|DEBUGHitActorLineTrace))

(event EventStopAction
  (CallFunction|ReleasePhotonBeam))

(event EventStartAction
  (CallFunction|ChargePhotonBeam))

(fn ConstructionScript)

(fn ChargePhotonBeam
  (bind _returnvalue (Audio|SpawnSound2D (Variables|Default|GetChargingSound) 1.0 1.0 0.0 0))
  (Variables|Default|SetChargingSoundComponent _returnvalue)
  (CallFunction|SetPhotonBeamValues (Variables|Default|GetChargeEndPoint) (Variables|Default|GetChargeBeamWidth) (Variables|Default|GetChargeNoiseFrequency) (Variables|Default|GetChargeNoiseCurve)))

(fn ReleasePhotonBeam
  (bind _chargingsoundcomponent (Variables|Default|GetChargingSoundComponent))
  (Utilities|IsValid _chargingsoundcomponent
    (:Is%20Valid
      (Audio|Components|Audio|Stop _chargingsoundcomponent))
    (:Is%20Not%20Valid
      _))
  (CallFunction|SetPhotonBeamValues (Variables|Default|GetReleaseEndPoint) (Variables|Default|GetReleaseBeamWidth) (Variables|Default|GetReleaseNoiseFrequency) (Variables|Default|GetReleaseNoiseCurve))
  (Audio|SpawnSound2D (Variables|Default|GetReleaseSound) 1.0 1.0 0.0 0)
  (CallFunction|HitEnemy "None")
  (CallFunction|ResetPhotonBeamtoZero))

(fn SetPhotonBeamValues
  (params (EndPoint :type Vector) (Width :type Float%20%28double-precision%29) (NoiseFrequency :type Float%20%28double-precision%29) (NoiseCurve :type Float%20%28double-precision%29))
  (bind _ns_photonbeam (Variables|Default|GetNS_PhotonBeam))
  (Niagara|SetNiagaraVariable(Vector3) _ns_photonbeam "BeamEndpoint" EndPoint)
  (Niagara|SetNiagaraVariable(Float) _ns_photonbeam "BeamWidth" Width)
  (Niagara|SetNiagaraVariable(Float) _ns_photonbeam "NoiseFrequency" NoiseFrequency)
  (Niagara|SetNiagaraVariable(Float) _ns_photonbeam "NoiseCurve" NoiseCurve))

(fn HitEnemy
  (params (DrawDebugType :type EDrawDebugTrace%20Enum :default "None"))
  (bind _spawnlocationarrow (Variables|Default|GetSpawnLocationArrow))
  (bind _returnvalue (Transformation|GetWorldLocation _spawnlocationarrow))
  (bind _outhit (Collision|LineTraceByChannel _returnvalue (+ _returnvalue (* (Math|Vector|GetForwardVector (Transformation|GetWorldRotation _spawnlocationarrow)) 6e+03)) "TraceTypeQuery1" false 0 DrawDebugType))
  (Game|Damage|ApplyDamage (.HitActor (Collision|BreakHitResult _outhit)) 1.0 0 0))

(fn DEBUGHitActorLineTrace
  (bind _spawnlocationarrow (Variables|Default|GetSpawnLocationArrow))
  (bind _returnvalue (Transformation|GetWorldLocation _spawnlocationarrow))
  (bind _outhit (Collision|LineTraceByChannel _returnvalue (+ _returnvalue (* (Math|Vector|GetForwardVector (Transformation|GetWorldRotation _spawnlocationarrow)) 6e+03)) "TraceTypeQuery1" false 0 "ForOneFrame"))
  (Development|PrintString (Utilities|GetDisplayName (.HitActor (Collision|BreakHitResult _outhit)))))