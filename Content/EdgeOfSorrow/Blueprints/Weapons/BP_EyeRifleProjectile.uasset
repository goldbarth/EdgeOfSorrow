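; BP_EyeRifleProjectile is the projectile for the Eye Rifle weapon.
; Hitting a component that is not simulating physics plays an impact sound, applies damage, attaches a temporary bullet-hole decal and destroys the projectile.
; Once ChangeColor sets HasChanged, Tick creates a new dynamic material every frame with a changed emissive color.
; It applies that material to the first projectile found by GetAllActorsOfClass, not necessarily itself.
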(event Custom|ChangeColor
  (Variables|Default|SetHasChanged true))

(event EventTick
  (params (DeltaSeconds :type Float%20%28single-precision%29))
  (if (Variables|Default|GetHasChanged)
    (bind _returnvalue (Rendering|Material|CreateDynamicMaterialInstance "/Game/EdgeOfSorrow/Weapons/EyeRifle/Projectile/M_Projectile_Inst.M_Projectile_Inst" "None" "None" :!class /Script/Engine.KismetMaterialLibrary))
    (Variables|Default|SetProjectileMesh _returnvalue)
    (bind _outactors (Actor|GetAllActorsOfClass "BP_EyeRifleProjectile_C"))
    (Rendering|Material|SetMaterial (Variables|BP_EyeRifleProjectile_C|GetSphere (Utilities|Array|Get(acopy) _outactors)) 0 (Variables|Default|GetProjectileMesh))
    (Rendering|Material|SetVectorParameterValue (Variables|Default|GetProjectileMesh) "EmissiveColor" (Math|Conversions|ToLinearColor(Vector) (Math|Conversions|ToVector(LinearColor) "(R=0.771647,G=0.000000,B=1.000000,A=1.000000)")) :!class /Script/Engine.MaterialInstanceDynamic)))

(event Collision|EventHit
  (params (MyComp :type Primitive%20Component%20Object%20Reference) (Other :type Actor%20Object%20Reference) (OtherComp :type Primitive%20Component%20Object%20Reference) (bSelfMoved :type Boolean) (HitLocation :type Vector :default "0, 0, 0") (HitNormal :type Vector :default "0, 0, 0") (NormalImpulse :type Vector :default "0, 0, 0") (Hit :type Hit%20Result%20Structure%20%28by%20ref%29))
  ;[0 0 0] Destroy the object at any physics object we hit. Spawn a Decal and destroy the Projectile.
  (if (not (Physics|IsSimulatingPhysics OtherComp "None"))
    (Audio|PlaySoundatLocation "/Game/EdgeOfSorrow/Audio/GDC_GameAudio/heavy_hit.heavy_hit" HitLocation "0, 0, 0" 1.0 1.0 0.0 0 0 0 0)
    (Game|Damage|ApplyDamage Other 1.0 0 self)
    (Class|GameplayStatics|SpawnDecalAttached "/Game/EdgeOfSorrow/Weapons/EyeRifle/Materials/M_BulletHole.M_BulletHole" "22.000000,44.000000,44.000000" OtherComp "None" HitLocation (Math|Conversions|RotationFromXVector HitNormal) "KeepWorldPosition" 1e+01)
    (Actor|DestroyActor)))

(fn ConstructionScript)