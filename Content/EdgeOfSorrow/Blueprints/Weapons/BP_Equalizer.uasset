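; BP_Equalizer is a weapon Blueprint that zaps all actors carrying a configured tag with electric beams and damage.
; StartAction runs UpdateTraces, which, once the cooldown has elapsed, gathers the tagged actors and casts a random-direction Visibility trace from the spawn arrow for each.
; Any blocking hit spawns a Niagara beam toward that target's location, offset by the hit normal, and damages the target regardless of what the trace hit.
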(event EventStartAction
  (CallFunction|UpdateTraces))

(fn ConstructionScript)

(fn UpdateTraces
  (bind _spawnlocationarrow (Variables|Default|GetSpawnLocationArrow))
  (bind _returnvalue (Transformation|GetWorldLocation _spawnlocationarrow))
  (if (>= (- (Utilities|Time|GetTimeSeconds) (Variables|Default|GetLastTrace)) (Variables|Default|GetTraceCooldowm))
    (bind _outactors (Actor|GetAllActorswithTag (Variables|Default|GetTagName)))
    (bind _output_get (Variables|Default|SetTargets _outactors))
    (for _array_element _output_get
      (bind _output_get_2 (Variables|Default|SetTarget _array_element))
      (LocalVariables|SetTargetPoint (Transformation|GetActorLocation _output_get_2))
      (LocalVariables|SetRandomDirection (Math|Random|RandomUnitVector))
      (LocalVariables|SetStartPoint (* (LocalVariables|GetRandomDirection) (Variables|Default|GetMinRadius)))
      (LocalVariables|SetEndPoint (* (LocalVariables|GetRandomDirection) (Variables|Default|GetMaxRadius)))
      (bind _outhit (Collision|LineTraceByChannel (+ (* (LocalVariables|GetRandomDirection) (Variables|Default|GetMinRadius)) _returnvalue) (+ _returnvalue (* (LocalVariables|GetRandomDirection) (Variables|Default|GetMaxRadius))) "TraceTypeQuery1" false 0 "None" true "(R=0.000000,G=0.000000,B=0.000000,A=1.000000)" "(R=0.000000,G=1.000000,B=0.000000,A=1.000000)" (Variables|Default|GetTraceCooldowm)))
      (Variables|Default|SetLastTrace (Utilities|Time|GetTimeSeconds))
      (if (.bBlockingHit (Collision|BreakHitResult _outhit))
        (LocalVariables|SetImpactPoint (.ImpactPoint (Collision|BreakHitResult _outhit)))
        (LocalVariables|SetImpactNormal (.ImpactNormal (Collision|BreakHitResult _outhit)))
        (bind _returnvalue_2 (Niagara|SpawnSystemAttached "/Game/EdgeOfSorrow/Blueprints/Particles/NS_ElectricBeam.NS_ElectricBeam" (Variables|Default|GetDefaultSceneRoot) "None" "0, 0, 0" "0, 0, 0" "KeepRelativeOffset" true))
        (Niagara|SetNiagaraVariable(Vector3) _returnvalue_2 "StartPoint" (LocalVariables|GetStartPoint))
        (Niagara|SetNiagaraVariable(Vector3) _returnvalue_2 "EndPoint" (+ (LocalVariables|GetTargetPoint) (* (LocalVariables|GetImpactNormal) (LocalVariables|GetImpactOffset))))
        (Niagara|SetNiagaraVariable(Vector3) _returnvalue_2 "ImpactNormal" (LocalVariables|GetImpactNormal))
        (Game|Damage|ApplyDamage (Variables|Default|GetTarget) (Variables|Default|GetDamage) 0 0)))))