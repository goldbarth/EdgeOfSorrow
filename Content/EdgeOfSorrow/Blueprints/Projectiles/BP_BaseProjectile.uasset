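; BP_BaseProjectile is a base projectile that deals damage and leaves an impact decal when it hits something.
; On Hit it ignores actors tagged Player and components that simulate physics.
; Other hits play a heavy impact sound, apply Damage, attach a short-lived decal oriented to the surface normal, and destroy the projectile.
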(event Collision|EventHit
  (params (MyComp :type Primitive%20Component%20Object%20Reference) (Other :type Actor%20Object%20Reference) (OtherComp :type Primitive%20Component%20Object%20Reference) (bSelfMoved :type Boolean) (HitLocation :type Vector :default "0, 0, 0") (HitNormal :type Vector :default "0, 0, 0") (NormalImpulse :type Vector :default "0, 0, 0") (Hit :type Hit%20Result%20Structure%20%28by%20ref%29))
  ;[0 0 0] Destroy the object at any physics object we hit. Spawn a Decal and destroy the Projectile.
  (Variables|Default|SetHitLocation HitLocation)
  (if (not (Actor|ActorHasTag Other "Player"))
    (if (not (Physics|IsSimulatingPhysics OtherComp "None"))
      (Audio|PlaySoundatLocation "/Game/EdgeOfSorrow/Audio/GDC_GameAudio/SW_HeavyHit_Cue.SW_HeavyHit_Cue" (Variables|Default|GetHitLocation) "0, 0, 0" 1.0 1.0 0.0 0 0 0 0)
      (Game|Damage|ApplyDamage Other (Variables|Default|GetDamage) 0 self)
      (Class|GameplayStatics|SpawnDecalAttached (Variables|Default|GetDecal%20Material) (Variables|Default|GetDecal%20Size) OtherComp "None" (Variables|Default|GetHitLocation) (Math|Conversions|RotationFromXVector HitNormal) "KeepWorldPosition" 1e+01)
      (Actor|DestroyActor))))

(fn ConstructionScript)