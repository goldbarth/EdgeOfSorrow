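; Enemy spawner actor that spawns queued enemy classes at its own transform and can be destroyed by damage.
; A looping timer spawns the next queued enemy, and adding to the queue also spawns immediately if no BP_DollHead overlaps its capsule.
; Each spawn gets a delegate bound to its destroyed event, and OnEnemyDefeated forwards defeats to BP_FirstPersonGameMode.
; Incoming damage lowers Health, prints it, and destroys the spawner at zero.
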(event Custom|OnEnemyDefeated
  (bind _asbp_first_person_game_mode (Utilities|Casting|CastToBP_FirstPersonGameMode (Game|GetGameMode)))
  (Default|OnEnemyDefeated _asbp_first_person_game_mode))

(event Custom|TryToSpawn
  ;[0 0 0] Spawn loop
  (CallFunction|SpawnEnemy))

(event EventBeginPlay
  ;[0 0 0] Spawn loop
  (Utilities|Time|SetTimerbyEvent (delegate Custom|TryToSpawn) 2.0 true))

(event Game|Damage|EventAnyDamage
  (params (Damage :type Float%20%28single-precision%29) (DamageType :type Damage%20Type%20Object%20Reference) (InstigatedBy :type Controller%20Object%20Reference) (DamageCauser :type Actor%20Object%20Reference))
  ;[0 0 0] Damage logic
  (CallFunction|TakeDamage Damage))

(fn ConstructionScript)

(fn SpawnEnemy
  ;[0 0 0] Spawns enemies in the right time
  (if (Utilities|Array|IsValidIndex (Variables|Default|GetEnemyQueue))
    (bind _returnvalue (Game|SpawnActorfromClass (Utilities|Array|Get(acopy) (Variables|Default|GetEnemyQueue)) (Transformation|GetActorTransform) "Undefined" "MultiplyWithRoot" 0 0))
    (EventDispatchers|BindEventtoOnEnemyDestroyed _returnvalue (EventDispatchers|CreateEvent :!event Custom|OnEnemyDefeated))
    (Utilities|Array|RemoveIndex (Variables|Default|GetEnemyQueue))
    (return true)
    (else
      (return false))))

(fn AddEnemytoQueue
  (params (EnemyClass :type BP%20Doll%20Head%20Class%20Reference%20%28by%20ref%29))
  (Utilities|Array|Add (Variables|Default|GetEnemyQueue) EnemyClass)
  (if (not (Utilities|Array|IsValidIndex (Collision|GetOverlappingActors (Variables|Default|GetCapsuleCollision) "/Game/EdgeOfSorrow/Blueprints/BP_DollHead.BP_DollHead_C" :!class /Script/Engine.PrimitiveComponent)))
    (CallFunction|SpawnEnemy)))

(fn TakeDamage
  (params (B :type Float%20%28double-precision%29))
  (bind _output_get (Variables|Default|SetHealth (Math|Float|Truncate (- (Variables|Default|GetHealth) B))))
  (Development|PrintString (Utilities|String|ToString(Integer) _output_get) true false)
  (if (<= (Variables|Default|GetHealth) 0)
    (Actor|DestroyActor)))