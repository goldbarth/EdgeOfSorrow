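; Wave controller that spawns timed enemy waves from the placed level config and tells the arena game mode when the round ends.
; TryStartWave waits until no actors are tagged Enemy, then schedules the next wave after a random configured delay.
; Each wave has the spawn holder evaluate random spawn points, then spawns a random selected enemy type at each, binding its death event.
; A boss spawn function exists but is not called here.
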(event Custom|Start
  (CallFunction|NewWave))

(event Custom|TryStartWave
  (bind _currentlevelconfig (Variables|Default|GetCurrentLevelConfig))
  (bind _waveindex (Variables|Default|GetWaveIndex))
  (bind _waveconfigs (Variables|/Game/EdgeOfSorrow/Blueprints/WaveSystem/Config/BP_LevelConfig.BP_LevelConfig_C|GetWaveConfigs _currentlevelconfig))
  (bind _output (Utilities|Array|Get(acopy) _waveconfigs _waveindex))
  (bind _outactors (Actor|GetAllActorswithTag "Enemy"))
  (if (<= (Utilities|Array|Length _outactors) 0)
    (if (< (Variables|Default|GetWaveIndex) (Variables|/Game/EdgeOfSorrow/Blueprints/WaveSystem/Config/BP_LevelConfig.BP_LevelConfig_C|GetWaveCount (Variables|Default|GetCurrentLevelConfig)))
      (Utilities|IsValid _output
        (:Is%20Valid
          (Utilities|Time|SetTimerbyEvent (delegate Custom|Start) (Math|Random|RandomFloatinRange (Variables|/Game/EdgeOfSorrow/Blueprints/WaveSystem/Config/BP_WaveConfigDataAsset.BP_WaveConfigDataAsset_C|GetMinSpawnDelay _output) (Variables|/Game/EdgeOfSorrow/Blueprints/WaveSystem/Config/BP_WaveConfigDataAsset.BP_WaveConfigDataAsset_C|GetMaxSpawnDelay _output)))))
      (else
        (Default|OnRoundEnd (Variables|Default|GetArenaGameMode))))))

(event EventBeginPlay
  (Utilities|FlowControl|Sequence
    (:then_0
      (CallFunction|SetGameMode))
    (:then_1
      (CallFunction|SetSpawnHandler))
    (:then_2
      (CallFunction|SetLevelConfig))
    (:then_3
      (Utilities|FlowControl|Delay 3.0)
      (CallFunction|TryStartWave))))

(fn ConstructionScript)

(fn SetGameMode
  (bind _returnvalue (Game|GetGameMode))
  (bind _asbp_arena_game_mode (Utilities|Casting|CastToBP_ArenaGameMode _returnvalue))
  (Utilities|IsValid _asbp_arena_game_mode
    (:Is%20Valid
      (Variables|Default|SetArenaGameMode _asbp_arena_game_mode))))

(fn SpawnEnemy
  (params (SpawnPoint :type Actor%20Object%20Reference) (Enemies :type Map%20of%20E_SelectedEnemy%20Enums%20to%20Classs :default "NewEnumerator0") (SelectedEnemies :type Array%20of%20E_SelectedEnemy%20Enums :default "NewEnumerator0"))
  (bind _returnvalue (Game|SpawnActorfromClass (.Value (Utilities|Map|Find Enemies (.OutItem (Utilities|Array|Random SelectedEnemies)))) (Transformation|GetActorTransform SpawnPoint) "Undefined" "MultiplyWithRoot" 0 0))
  (Utilities|IsValid _returnvalue
    (:Is%20Valid
      (EventDispatchers|BindEventtoOnEnemyDeath _returnvalue (EventDispatchers|CreateEvent :!event Custom|TryStartWave)))))

(fn SpawnEnemyBoss
  (params (SpawnPoint :type Actor%20Object%20Reference) (Enemies :type Map%20of%20E_SelectedEnemy%20Enums%20to%20Classs :default "NewEnumerator0") (EnemyBoss :type E_SelectedEnemy%20Enum :default "NewEnumerator0"))
  (if (Utilities|Enum|NotEqual(Enum) EnemyBoss "NewEnumerator6")
    (bind _returnvalue (Game|SpawnActorfromClass (.Value (Utilities|Map|Find Enemies EnemyBoss)) (Transformation|GetActorTransform SpawnPoint) "Undefined" "MultiplyWithRoot" 0 0))
    (EventDispatchers|BindEventtoOnEnemyDeath _returnvalue (EventDispatchers|CreateEvent :!event Custom|TryStartWave))))

(fn Wave
  (params (CurrentWaveConfig :type BP%20Wave%20Config%20Data%20Asset%20Object%20Reference))
  (bind _output_get (LocalVariables|SetConfig CurrentWaveConfig))
  (Utilities|IsValid _output_get
    (:Is%20Valid
      (Utilities|IsValid (Variables|Default|GetSpawnHolder)
        (:Is%20Valid
          (Default|EvaluateRandomSpawnPoints (Variables|Default|GetSpawnHolder) (Variables|/Game/EdgeOfSorrow/Blueprints/WaveSystem/Config/BP_WaveConfigDataAsset.BP_WaveConfigDataAsset_C|GetEnemyCount (LocalVariables|GetConfig)) (Variables|/Game/EdgeOfSorrow/Blueprints/WaveSystem/Config/BP_WaveConfigDataAsset.BP_WaveConfigDataAsset_C|GetMinRadius (LocalVariables|GetConfig)) (Variables|/Game/EdgeOfSorrow/Blueprints/WaveSystem/Config/BP_WaveConfigDataAsset.BP_WaveConfigDataAsset_C|GetMaxRadius (LocalVariables|GetConfig)))
          (bind _outactors (Actor|GetAllActorsOfClass "/Game/EdgeOfSorrow/Blueprints/WaveSystem/BP_SpawnPoint.BP_SpawnPoint_C"))
          (for _array_element _outactors
            (CallFunction|SpawnEnemy _array_element (Variables|/Game/EdgeOfSorrow/Blueprints/WaveSystem/Config/BP_WaveConfigDataAsset.BP_WaveConfigDataAsset_C|GetEnemies (LocalVariables|GetConfig)) (Variables|/Game/EdgeOfSorrow/Blueprints/WaveSystem/Config/BP_WaveConfigDataAsset.BP_WaveConfigDataAsset_C|GetSelectedEnemies (LocalVariables|GetConfig)))))))))

(fn NewWave
  (CallFunction|Wave (Utilities|Array|Get(acopy) (Variables|/Game/EdgeOfSorrow/Blueprints/WaveSystem/Config/BP_LevelConfig.BP_LevelConfig_C|GetWaveConfigs (Variables|Default|GetCurrentLevelConfig)) (Variables|Default|GetWaveIndex)))
  (Math|Integer|IncrementInt (Variables|Default|GetWaveIndex)))

(fn SetLevelConfig
  (bind _outactors (Actor|GetAllActorsOfClass "/Game/EdgeOfSorrow/Blueprints/WaveSystem/Config/BP_LevelConfig.BP_LevelConfig_C"))
  (Variables|Default|SetCurrentLevelConfig (Utilities|Array|Get(acopy) _outactors)))

(fn SetSpawnHandler
  (bind _outactors (Actor|GetAllActorsOfClass "/Game/EdgeOfSorrow/Blueprints/WaveSystem/BP_SpawnHolder.BP_SpawnHolder_C"))
  (Utilities|IsValid (Utilities|Array|Get(acopy) _outactors)
    (:Is%20Valid
      (Variables|Default|SetSpawnHolder (Utilities|Array|Get(acopy) _outactors)))))