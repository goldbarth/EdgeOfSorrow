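; BP_SpawnHolder is a wave-system actor that creates and repositions enemy or wave spawn points using the player's location.
; On BeginPlay it caches the first-person character and adds a configured number of BP_SpawnPoint child actor components.
; EvaluateRandomSpawnPoints, not called here, moves each to a random "donut" position at player height.
; That math adds player X/Y to the radius before the cosine/sine multiply, so the ring is not truly player-centred.
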(event EventBeginPlay
  (Utilities|FlowControl|Sequence
    (:then_0
      (CallFunction|SetFirstPersonCharacter))
    (:then_1
      (CallFunction|SetStartSpawnPoints))))

(fn ConstructionScript)

(fn SetFirstPersonCharacter
  (bind _returnvalue (Game|GetPlayerCharacter 0))
  (bind _asbp_first_person_character (Utilities|Casting|CastToBP_FirstPersonCharacter _returnvalue))
  (Utilities|IsValid _asbp_first_person_character
    (:Is%20Valid
      (Variables|Default|SetFirstPersonCharacter _asbp_first_person_character))))

(fn SetStartSpawnPoints
  (for _index (range 0 (- (Variables|Default|GetStartSpawnPoints) 1))
    (CallFunction|AddSpawnPoint)))

(fn AddSpawnPoint
  (bind _returnvalue (AddComponent|AddChildActorComponent false))
  (bind _output_get (Variables|Default|SetChildActor _returnvalue))
  (ChildActorComponent|SetChildActorClass _output_get "/Game/EdgeOfSorrow/Blueprints/WaveSystem/BP_SpawnPoint.BP_SpawnPoint_C")
  (Utilities|Array|Add (Variables|Default|GetSpawnPoints) (Variables|Default|GetChildActor)))

(fn SetRandomPosition
  (bind _firstpersoncharacter (Variables|Default|GetFirstPersonCharacter))
  (bind _returnvalue (Transformation|GetActorLocation _firstpersoncharacter))
  (Variables|Default|SetRandomAngle (Math|Random|RandomFloatinRange 0.0 3.6e+02))
  (Variables|Default|SetRandomRadius (Math|Random|RandomFloatinRange (Variables|Default|GetMinRadius) (Variables|Default|GetMaxRadius)))
  (bind _output_get (Variables|Default|SetSpawnLocation (Math|Vector|MakeVector (* (+ (.x _returnvalue) (Variables|Default|GetRandomRadius)) (Math|Trig|Cos(Degrees) (Variables|Default|GetRandomAngle))) (* (+ (.y _returnvalue) (Variables|Default|GetRandomRadius)) (Math|Trig|Sin(Degrees) (Variables|Default|GetRandomAngle))) (.z _returnvalue))))
  (return _output_get))

(fn EvaluateRandomSpawnPoints
  (for _array_element (Variables|Default|GetSpawnPoints)
    (bind _spawnposition (CallFunction|SetRandomPosition))
    (Transformation|SetWorldLocation _array_element _spawnposition false false)))