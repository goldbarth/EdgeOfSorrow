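; BP_PostProcessVolumeHolder manages the darkness post process volumes, which vary with the game's difficulty.
; On BeginPlay it caches BP_GameInstance, then enables the player darkness volume matching CurrentDifficulty (Easy, Medium or Hard).
; SwitchLightPosition disables that difficulty's player volume and enables the darkness exit volume in its place.
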(event EventBeginPlay
  (Utilities|FlowControl|Sequence
    (:then_0
      (CallFunction|SetGameInstance))
    (:then_1
      (CallFunction|SetDifficultyShadowDistance))))

(fn ConstructionScript)

(fn SwitchLightPosition
  (Variables|/Script/Engine.PostProcessComponent|SetbEnabled (Utilities|Select :Index (Variables|/Game/EdgeOfSorrow/Blueprints/BP_GameInstance.BP_GameInstance_C|GetCurrentDifficulty (Variables|Default|GetGameInstance)) :NewEnumerator0 (Variables|Default|GetDarknessPlayerEasyPPV) :NewEnumerator1 (Variables|Default|GetDarknessPlayerMediumPPV) :NewEnumerator2 (Variables|Default|GetDarknessPlayerHardPPV)) false)
  (Variables|/Script/Engine.PostProcessComponent|SetbEnabled (Variables|Default|GetDarknessExitPPV) true))

(fn SetGameInstance
  (bind _returnvalue (Game|GetGameInstance))
  (bind _asbp_game_instance (Utilities|Casting|CastToBP_GameInstance _returnvalue))
  (Utilities|IsValid _asbp_game_instance
    (:Is%20Valid
      (Variables|Default|SetGameInstance _asbp_game_instance))))

(fn SetDifficultyShadowDistance
  (Variables|/Script/Engine.PostProcessComponent|SetbEnabled (Utilities|Select :Index (Variables|/Game/EdgeOfSorrow/Blueprints/BP_GameInstance.BP_GameInstance_C|GetCurrentDifficulty (Variables|Default|GetGameInstance)) :NewEnumerator0 (Variables|Default|GetDarknessPlayerEasyPPV) :NewEnumerator1 (Variables|Default|GetDarknessPlayerMediumPPV) :NewEnumerator2 (Variables|Default|GetDarknessPlayerHardPPV)) true))