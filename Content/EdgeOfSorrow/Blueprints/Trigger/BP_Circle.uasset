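; BP_Circle is a ruins circle trigger that exits the arena level once the round is won.
; OnRoundWon_Event makes it vulnerable, swapping both mesh materials and setting a flag.
; A sphere collision hit from a Player-tagged actor then calls EndLevel on BP_ArenaGameMode to go to "Shop"; other actors only print a taunt.
; The enemy-tag check is disconnected, and CheckEnemyCount is not called here.
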(event OnComponentHit(SphereCollision)
  (params (HitComponent :type Primitive%20Component%20Object%20Reference) (OtherActor :type Actor%20Object%20Reference) (OtherComp :type Primitive%20Component%20Object%20Reference) (NormalImpulse :type Vector :default "0, 0, 0") (Hit :type Hit%20Result%20Structure%20%28by%20ref%29))
  (Utilities|IsValid OtherActor
    (:Is%20Valid
      (if (Variables|Default|GetIsVunerable)
        (if (not (Actor|ActorHasTag OtherActor "Player"))
          (Development|PrintString "NICE TRY PASCAL :P" true true "(R=0.000000,G=1.000000,B=0.056510,A=1.000000)" 1e+01)
          (else
            (Default|EndLevel (.AsBP%20Arena%20Game%20Mode (Utilities|Casting|CastToBP_ArenaGameMode (Game|GetGameMode))) "Shop")))))))

(event Custom|OnRoundWon_Event
  (CallFunction|SetVulnerable)
  (Development|PrintString "ALL ENEMIES ARE DEAD" true true "(R=0.015626,G=1.000000,B=0.000000,A=1.000000)"))

(event Custom|TestEvent)

(event EventTick
  (params (DeltaSeconds :type Float%20%28single-precision%29)))

(fn ConstructionScript)

(fn CheckEnemyCount
  (params (ActorClass :type Actor%20Class%20Reference))
  (bind _outactors (Actor|GetAllActorsOfClass ActorClass))
  (return (<= (Utilities|Array|Length _outactors) 0)))

(fn SetVulnerable
  (Rendering|Material|SetMaterial (Variables|Default|GetSM_RuinsCircle) 0 "/Game/EdgeOfSorrow/Materials/CelColors/M_CelColor4.M_CelColor4")
  (Rendering|Material|SetMaterial (Variables|Default|GetSM_RuinsCircle) 1 "/Game/EdgeOfSorrow/Materials/CelColors/M_CelColor4.M_CelColor4")
  (Variables|Default|SetIsVunerable true))